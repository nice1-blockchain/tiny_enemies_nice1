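; BP_Unit is a team-colored 2D Paper flipbook unit that belongs to a wave parent and tracks a killed flag.
; On BeginPlay it tints itself from the wave's team, attaches an extra sprite if tagged special, and delays enabling its stimulus collider for overlaps.
; A looping, start-staggered timer refreshes Z-order.
; Update8Way swaps directional walk flipbooks at a random frame.
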(event Custom|Update8Way
  (params (8WayDirection :type Integer))
  (Sprite|SetFlipbook (Variables|Default|GetPaperFlipbook) (Utilities|Select :Index 8WayDirection :Option%200 "/Game/Tiny/Art/Game/Sprites/PFB_Unit_Walk_D6.PFB_Unit_Walk_D6" :Option%201 "/Game/Tiny/Art/Game/Sprites/PFB_Unit_Walk_D3.PFB_Unit_Walk_D3" :Option%202 "/Game/Tiny/Art/Game/Sprites/PFB_Unit_Walk_D2.PFB_Unit_Walk_D2" :Option%203 "/Game/Tiny/Art/Game/Sprites/PFB_Unit_Walk_D1.PFB_Unit_Walk_D1" :Option%204 "/Game/Tiny/Art/Game/Sprites/PFB_Unit_Walk_D4.PFB_Unit_Walk_D4" :Option%205 "/Game/Tiny/Art/Game/Sprites/PFB_Unit_Walk_D7.PFB_Unit_Walk_D7" :Option%206 "/Game/Tiny/Art/Game/Sprites/PFB_Unit_Walk_D8.PFB_Unit_Walk_D8" :Option%207 "/Game/Tiny/Art/Game/Sprites/PFB_Unit_Walk_D9.PFB_Unit_Walk_D9" :Option%208 "/Game/Tiny/Art/Game/Sprites/PFB_Unit_Walk_D6.PFB_Unit_Walk_D6"))
  (Class|PaperFlipbookComponent|SetPlaybackPositioninFrames (Variables|Default|GetPaperFlipbook) (Math|Random|RandomIntegerinRange 0 7) false))

(event Custom|UpdateZOrder
  (CallFunction|UpdateZOrder (Variables|Default|GetPaperFlipbook)))

(event EventBeginPlay
  (Utilities|FlowControl|Sequence
    (:then_0
      (if true ; Set team color.
        (Sprite|SetSpriteColor (Variables|Default|GetPaperFlipbook) (CallFunction|GetTeamColor (Default|GetTeamValue (Variables|/Game/Tiny/Blueprints/BP_Wave.BP_Wave_C|GetAC_Team (Variables|Default|GetBP_Wave_Parent)))))))
    (:then_1
      (if true ; Special unit.
        (if (GameplayTags|MatchesTag (Variables|Default|GetSpecialUnit) "(TagName=\"Unit.Special\")")
          (bind _returnvalue (AddComponent|AddPaperSpriteComponent true (Math|Transform|MakeTransform "0, 0, 0" "0, 0,-90.000000" "1.000000,1.000000,1.000000")))
          (Transformation|AttachComponentToComponent _returnvalue (Variables|Default|GetPaperFlipbook) "None" "KeepRelative" "KeepWorld" "KeepRelative" true))))
    (:then_2
      (if true ; Update ZOrder.
        (Utilities|Time|SetTimerbyEvent (delegate Custom|UpdateZOrder) 0.25 true 0.0 0.1)))
    (:then_3
      (if true ; Overlap triggers delay.
        (Utilities|FlowControl|Delay 0.5)
        (Collision|SetCollisionEnabled (Variables|Default|GetStimulusCollider) "QueryOnly")))))

(fn ConstructionScript)

(fn GetKilled
  (return (Variables|Default|GetbKilled)))

(fn SetKilled
  (Variables|Default|SetbKilled true))