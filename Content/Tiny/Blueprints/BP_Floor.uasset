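; BP_Floor is a floor actor whose appearance and size are configured per instance through InitialImage and InitialScale.
; The Construction Script creates a dynamic instance of M_Unlit, sets its Texture parameter to InitialImage, and applies it to the static mesh.
; It then multiplies the mesh's current world scale by InitialScale.
; The event graph holds only disabled placeholder events, so it adds no runtime logic.
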(event EventBeginPlay)

(event Collision|EventActorBeginOverlap
  (params (OtherActor :type Actor%20Object%20Reference)))

(event EventTick
  (params (DeltaSeconds :type Float%20%28single-precision%29)))

(fn ConstructionScript
  (Utilities|FlowControl|Sequence
    (:then_0
      (bind _returnvalue (Rendering|Material|CreateDynamicMaterialInstance "/Game/Tiny/Art/M_Unlit.M_Unlit" "None" "None" :!class /Script/Engine.KismetMaterialLibrary))
      (Rendering|Material|SetTextureParameterValue _returnvalue "Texture" (Variables|InitialExposedValues|GetInitialImage))
      (Rendering|Material|SetMaterial (Variables|Default|GetStaticMesh) 0 _returnvalue))
    (:then_1
      (Transformation|SetWorldScale3D (Variables|Default|GetStaticMesh) (* (Transformation|GetWorldScale (Variables|Default|GetStaticMesh)) (Math|Conversions|ToVector(Float) (Variables|InitialExposedValues|GetInitialScale)))))))