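; BP_Wave is an AI pawn that carries one row of a team's units to a target camp.
; It staggers its start by row index, pathfinds with AIMoveTo, and spawns BP_Units attached to spread-out scene components.
; Tick updates units' 8-way facing from velocity and collapses the spread near the goal.
; On arrival a timer drains population into the camp as reinforcement or attack until depleted; kills en route reduce population and multicast shot FX.
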(event Custom|ToTower
  (bind _camp (Default|GetCamp (Variables|Refs|GetGS) (Variables|InitialExposedReplicatedValues|GetTowerEnd)))
  (bind (_bdepleted _extracted) (Default|Extract (Variables|Refs|GetAC_Population) (.Value (CallFunction|GetWavetoCampTransferSpeed))))
  (Utilities|FlowControl|Sequence
    (:then_0
      (if (== (Variables|InitialExposedReplicatedValues|GetInitialTeam) (Default|GetTeamValue (Variables|/Game/Tiny/Blueprints/BP_Camp.BP_Camp_C|GetAC_Team _camp)))
        (Default|Inject (Variables|/Game/Tiny/Blueprints/BP_Camp.BP_Camp_C|GetAC_Population _camp) _extracted)
        (else
          (Default|Income _camp (Variables|InitialExposedReplicatedValues|GetInitialTeam) _extracted (Variables|InitialExposedReplicatedValues|GetAtackMultiplier)))))
    (:then_1
      (if _bdepleted
        (Default|WaveDestroy (Variables|Refs|GetGS) self)))))

(event Custom|Arrive
  (Utilities|Time|SetTimerbyEvent (delegate Custom|ToTower) (.Seconds (CallFunction|GetWavetoCampTransferSpeed)) true))

(event Custom|MulticastUnitKilledFX
  (params (CampIndex :type Integer) (UnitIndex :type Integer))
  (bind _camp (Default|GetCamp (Variables|Refs|GetGS) CampIndex))
  (Default|ShootFX _camp (Utilities|Array|Get(acopy) (Variables|Private|GetBP_Units) UnitIndex)))

(event Custom|UnitKilled
  (params (CampIndex :type Integer) (UnitIndex :type Integer))
  (Default|Extract (Variables|Refs|GetAC_Population) 1.0)
  (CallFunction|MulticastUnitKilledFX CampIndex UnitIndex))

(event EventBeginPlay
  (bind _separationcm (CallFunction|GetWaveRowUnitSeparation))
  (bind _initialpopulation (Variables|InitialExposedReplicatedValues|GetInitialPopulation))
  (Utilities|FlowControl|Sequence
    (:then_0
      (if true
        (bind _asbp_gs_game (CallFunction|GetGSGame))
        (Variables|Refs|SetGS _asbp_gs_game)))
    (:then_1
      (if true ; Set SCToChase spread
        (for _index (range 0 (- _initialpopulation 1))
          (bind _returnvalue (AddComponent|AddSceneComponent false (Math|Transform|MakeTransform (Math|Vector|MakeVector 0.0 (- (* _index _separationcm) (* _separationcm (* _initialpopulation 0.5))) 0.0) "0, 0, 0" "1.000000,1.000000,1.000000")))
          (Utilities|Array|Add (Variables|Private|GetSCToChase) _returnvalue))))
    (:then_2
      (if true ; Delay wave init.
        (Utilities|FlowControl|Delay (* (- (Variables|InitialExposedReplicatedValues|GetRowIndex) 1) (CallFunction|GetWaveRowSeparation)))
        (Utilities|FlowControl|Sequence
          (:then_0
            (Variables|/Script/Engine.FloatingPawnMovement|SetMaxSpeed (Variables|Default|GetFloatingPawnMovement) (CallFunction|GetWaveSpeed)))
          (:then_2
            (if true ; AI Path Find
              (bind _camp (Default|GetCamp (Variables|Refs|GetGS) (Variables|InitialExposedReplicatedValues|GetTowerEnd)))
              (bind _output_get (Variables|Private|SetGoalLocation (Transformation|GetWorldLocation (Variables|/Game/Tiny/Blueprints/BP_Camp.BP_Camp_C|GetRoot _camp))))
              (AI|AIMoveTo (AI|GetAIController self) _output_get 0 (CallFunction|GetCampGoalRadius) "Disable" "Disable" true false
                (:OnMoveFinished
                  (CallFunction|Arrive)))))
          (:then_3
            (if true ; Spawn Units.
              (UnitSprites|SetTotalUnits)))
          (:then_4
            (if true ; Start tick.
              (Actor|Tick|SetActorTickEnabled true))))))))

(event EventTick
  (params (DeltaSeconds :type Float%20%28single-precision%29))
  (bind _floatingpawnmovement (Variables|Default|GetFloatingPawnMovement))
  (bind _velocity (Variables|/Script/Engine.MovementComponent|GetVelocity _floatingpawnmovement))
  (bind _yaw (Math|Vector|GetYawPitchfromVector _velocity))
  (bind _returnvalue (Class|KismetMathLibrary|ClampAxis _yaw))
  (bind _returnvalue_2 (Math|Float|MapRangeUnclamped _returnvalue 0.0 3.6e+02 0.5 8.5))
  (bind _returnvalue_3 (Math|Float|Truncate _returnvalue_2))
  (Utilities|FlowControl|Delay 0.2)
  (Utilities|FlowControl|Sequence
    (:then_0
      (if (> (Math|Vector|VectorLength _velocity) 2e+01)
        (Transformation|SetWorldRotation (Variables|Default|GetRoot) (Math|Rotator|MakeRotator 0.0 0.0 _yaw) false true)
        (if (!= (Variables|Private|Get8WayDirection) _returnvalue_3)
          (Variables|Private|Set8WayDirection _returnvalue_3)
          (for _array_element (Variables|Private|GetBP_Units)
            (Utilities|IsValid _array_element
              (:Is%20Valid
                (Default|Update8Way _array_element (Variables|Private|Get8WayDirection))))))))
    (:then_1
      (if (< (Math|Vector|VectorLength (- (Transformation|GetWorldLocation (Variables|Default|GetRoot)) (Variables|Private|GetGoalLocation))) 5e+01)
        (for _array_element_2 (Variables|Private|GetSCToChase)
          (Transformation|SetRelativeLocation _array_element_2 "0, 0, 0" false false))))))

(event EventEndPlay
  (params (EndPlayReason :type EEndPlayReason%20Enum :default "Destroyed"))
  (for _array_element (Variables|Private|GetBP_Units)
    (Utilities|IsValid _array_element
      (:Is%20Valid
        (Actor|DestroyActor _array_element)))))

(fn ConstructionScript
  (Default|SetTeamValue (Variables|Default|GetAC_Team) (Variables|InitialExposedReplicatedValues|GetInitialTeam))
  (Default|Inject (Variables|Refs|GetAC_Population) (Math|Conversions|ToFloat(Integer) (Variables|InitialExposedReplicatedValues|GetInitialPopulation))))

(fn SetTotalUnits
  (for _index (range 0 (- (.Truncated (Default|GetValue (Variables|Refs|GetAC_Population))) 1))
    (if (not (Utilities|Array|IsValidIndex (Variables|Private|GetBP_Units) _index))
      (UnitSprites|AddUnitActor _index))))

(fn AddUnitActor
  (params (Index :type Integer))
  (bind _returnvalue (Game|SpawnActorfromClass "/Game/Tiny/Blueprints/BP_Unit.BP_Unit_C" (Math|Transform|MakeTransform (Transformation|GetWorldLocation (Variables|Default|GetCrowd)) "0, 0, 0" "1.000000,1.000000,1.000000") "Undefined" 0 self Index 0))
  (if true ; Mind the overlap triggers firing here!
    (Utilities|Array|Add (Variables|Private|GetBP_Units) _returnvalue)
    (Transformation|AttachComponentToComponent _returnvalue (Utilities|Array|Get(acopy) (Variables|Private|GetSCToChase) Index) "None" "SnapToTarget" "KeepWorld" "KeepWorld" true)))