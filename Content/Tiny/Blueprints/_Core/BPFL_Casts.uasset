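; Blueprint function library of shared shortcuts for fetching typed game framework objects and data table rows in the Tiny game.
; Getters cast the game instance, Lobby and Game modes, states and controllers, and the Game player state, printing an error on failure; player lookups always use index 0.
; Table getters build row names from a world tag, camp type and level, or level to read Worlds, Upgrade, Grow and Shoot rows.
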(fn GetGI
  (bind _asgi_tiny (Utilities|Casting|CastToGI_Tiny (Game|GetGameInstance))
    (:then
      (return _asgi_tiny))
    (:CastFailed
      (Development|PrintString 0 "GI  Cast failed!"))))

(fn GetGMLobby
  (bind _asgm_lobby (Utilities|Casting|CastToGM_Lobby (Game|GetGameMode))
    (:then
      (return _asgm_lobby))
    (:CastFailed
      (Development|PrintString 0 "GM Cast failed!"))))

(fn GetGSLobby
  (bind _asgs_lobby (Utilities|Casting|CastToGS_Lobby (Game|GetGameState))
    (:then
      (return _asgs_lobby))
    (:CastFailed
      (Development|PrintString 0 "GM Cast failed!"))))

(fn GetPCLobby
  (bind _aspc_lobby (Utilities|Casting|CastToPC_Lobby (Game|GetPlayerController 0))
    (:then
      (return _aspc_lobby))
    (:CastFailed
      (Development|PrintString 0 "PC Cast failed!"))))

(fn GetGMGame
  (bind _asgm_game (Utilities|Casting|CastToGM_Game (Game|GetGameMode))
    (:then
      (return _asgm_game))
    (:CastFailed
      (Development|PrintString 0 "GM Cast failed!"))))

(fn GetGSGame
  (bind _asgs_game (Utilities|Casting|CastToGS_Game (Game|GetGameState))
    (:then
      (return _asgs_game))
    (:CastFailed
      (Development|PrintString 0 "PC Cast failed!"))))

(fn GetPCGame
  (bind _aspc_game (Utilities|Casting|CastToPC_Game (Game|GetPlayerController 0))
    (:then
      (return _aspc_game))
    (:CastFailed
      (Development|PrintString 0 "PC Cast failed!"))))

(fn GetPSGame
  (bind _asps_game (Utilities|Casting|CastToPS_Game (Game|GetPlayerState 0))
    (:then
      (return _asps_game))
    (:CastFailed
      (Development|PrintString 0 "PS Cast failed!"))))

(fn GetDTWorldMap
  (params (World :type Gameplay%20Tag%20Structure))
  (bind _returnvalue (Utilities|GetDataTableRow "/Game/Tiny/Data/Worlds/DT_Worlds.DT_Worlds" (GameplayTags|GetTagName World))
    (:then
      (return _returnvalue))))

(fn GetDTUpgrade
  (params (Camp :type S%20Camp%20Structure))
  (bind (_type _level) (Utilities|Struct|BreakSCamp Camp))
  (bind _returnvalue (Utilities|GetDataTableRow "/Game/Tiny/Data/Camps/DT_Upgrade.DT_Upgrade" (Utilities|String|StringToName (Utilities|String|Append (GameplayTags|GetDebugStringfromGameplayTag _type) "." (Utilities|String|ToString(Integer) _level))))
    (:then
      (return _returnvalue))))

(fn GetDTGrowbyLevel
  (params (Level :type Integer))
  (bind _returnvalue (Utilities|GetDataTableRow "/Game/Tiny/Data/Camps/DT_Grow.DT_Grow" (Utilities|String|StringToName (Utilities|String|Append "Level_" (Utilities|String|ToString(Integer) Level))))
    (:then
      (return _returnvalue))))

(fn GetDTShoot
  (params (Level :type Integer))
  (bind _returnvalue (Utilities|GetDataTableRow "/Game/Tiny/Data/Camps/DT_Shoot.DT_Shoot" (Utilities|String|StringToName (Utilities|String|ToString(Integer) Level)))
    (:then
      (return _returnvalue))))