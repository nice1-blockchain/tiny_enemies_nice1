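; PC_Menu is the player controller for the main menu, setting up the local player's menu environment on BeginPlay.
; A sequence sets game-and-UI input mode with an Enhanced Input mappable config, then creates or reuses the WBP_Menu widget and adds it to the viewport.
; It then has the game instance dispatch errors, destroys any session while printing the result, and starts the menu music through the game instance.
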(event EventBeginPlay
  (if (Pawn|IsLocalPlayerController)
    (Utilities|FlowControl|Sequence
      (:then_0
        (if true ; Input mode.
          (Input|SetInputModeGameandUI self 0 "DoNotLock" false)
          (Class|EnhancedInputSubsystemInterface|AddPlayerMappableConfig (PlayerController|LocalPlayerSubsystems|GetEnhancedInputLocalPlayerSubsystem) "/Game/Tiny/Data/Inputs/PBIC_PlayerInputs.PBIC_PlayerInputs" "(bIgnoreAllPressedKeysUntilRelease=True,bForceImmediately=False)")))
      (:then_1
        (if true ; UMG.
          (bind _wbp_main (Variables|Default|GetWBP_Main)
            (:then
              (if (not (UserInterface|Viewport|IsinViewport _wbp_main))
                (UserInterface|Viewport|AddtoViewport (Variables|Default|GetWBP_Main) 0 :!label _label)))
            (:else
              (bind _returnvalue (UserInterface|CreateWidget "/Game/Tiny/UI/Menu/WBP_Menu.WBP_Menu_C"))
              (Variables|Default|SetWBP_Main _returnvalue)
              (goto _label)))))
      (:then_2
        (if true ; Error check.
          (Default|DispatchErrors (CallFunction|GetGI))))
      (:then_3
        (if true ; Destroy session.
          (|DestroySession (Game|GetPlayerController 0)
            (:OnSuccess
              (Development|PrintString "Session destroyed."))
            (:OnFailure
              (Development|PrintString "Session destroyed. FAILURE")))))
      (:then_4
        (if true ; Music.
          (Default|PlayMusic (CallFunction|GetGI) "/Game/Tiny/Art/Audio/A_MenuMainMusic_Cue.A_MenuMainMusic_Cue"))))))

(fn ConstructionScript)