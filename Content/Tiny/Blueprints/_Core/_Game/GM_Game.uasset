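; GM_Game is the in-match game mode that gathers connecting players, starts the game when all are ready and handles the return to the lobby.
; Post-login and seamless-travel controller swaps register each PC_Game and bind its PC-ready event.
; Ready players and their profiles are counted against the current map's data-table player count before GS_Game starts the match.
; Logouts notify GS_Game; lobby travel clears widgets, then calls ServerTravel.
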(event Custom|TravelToLobby
  (Utilities|FlowControl|Sequence
    (:then_0
      (for _array_element (Variables|Default|GetAll_PC's)
        (bind _aspc_game (Utilities|Casting|CastToPC_Game _array_element))
        (Default|OCRemoveWidgets _aspc_game)))
    (:then_1
      (bind _returnvalue (Class|AdvancedSessionsLibrary|ServerTravel (Class|BlueprintPathsLibrary|GetBaseFilename (Utilities|ToString(SoftObjectReference) (Utilities|Select :Index 0 :Option%200 "/Game/Tiny/Maps/Menu/Lobby.Lobby" :Option%201 "/Game/Tiny/Maps/Menu/Lobby.Lobby")) true) true false))
      (if _returnvalue
        (Development|PrintString "Launching game... ")
        (else
          (Development|PrintString "Server travel fail."))))))

(event EventBeginPlay
  (bind _returnvalue (Game|GetCurrentLevelName true))
  (bind _world (CallFunction|GetWorldTagfromMapName _returnvalue))
  (bind _sworld (CallFunction|GetDTWorldMap _world))
  (Variables|Default|SetWorldPlayers (.Players (Utilities|Struct|BreakSWorld _sworld))))

(event EventPostLogin
  (params (NewPlayer :type Player%20Controller%20Object%20Reference))
  (bind _pcgame (CallFunction|PlayerConnect NewPlayer))
  (EventDispatchers|BindEventtoPCReady _pcgame (EventDispatchers|CreateEvent :!event PlayerReady)))

(event EventOnSwapPlayerControllers
  (params (OldPC :type Player%20Controller%20Object%20Reference) (NewPC :type Player%20Controller%20Object%20Reference))
  (bind _pcgame (CallFunction|PlayerConnect NewPC))
  (EventDispatchers|BindEventtoPCReady _pcgame (EventDispatchers|CreateEvent :!event PlayerReady)))

(event EventOnLogout
  (params (ExitingController :type Controller%20Object%20Reference))
  (bind _pc (CallFunction|PlayerDisconnect ExitingController))
  (EventDispatchers|UnbindallEventsfromPCReady _pc))

(fn ConstructionScript
  (|CallParentFunction))

(fn PlayerConnect
  (params (PC :type Player%20Controller%20Object%20Reference))
  (bind _aspc_game (Utilities|Casting|CastToPC_Game PC))
  (Utilities|Array|Add (Variables|Default|GetAll_PC's) _aspc_game)
  (return _aspc_game))

(fn PlayerDisconnect
  (params (Player :type Object%20Object%20Reference))
  (bind _aspc_game (Utilities|Casting|CastToPC_Game Player))
  (Utilities|FlowControl|Sequence
    (:then_0
      (Math|Integer|DecrementInt (Variables|Default|GetPlayersReady)))
    (:then_1
      (bind _asbp_gs_game (CallFunction|GetGSGame))
      (Default|PlayerAbandoned _asbp_gs_game _aspc_game))
    (:then_2
      (Utilities|Array|RemoveItem (Variables|Default|GetAll_PC's) _aspc_game)
      (return _aspc_game))))

(fn PlayerReady
  (params (PlayerController :type Player%20Controller%20Object%20Reference) (UserProfile :type S%20User%20Profile%20Structure))
  (Utilities|Map|Add (Variables|Default|GetAllProfiles) PlayerController UserProfile)
  (Math|Integer|IncrementInt (Variables|Default|GetPlayersReady)
    (:%20%20
      (CallFunction|CheckAllReady))))

(fn CheckAllReady
  (if (== (Variables|Default|GetWorldPlayers) (Variables|Default|GetPlayersReady))
    (bind _asbp_gs_game (CallFunction|GetGSGame))
    (Default|SRVStartGame _asbp_gs_game (Variables|Default|GetAll_PC's))
    (bind _values (Utilities|Map|Values (Variables|Default|GetAllProfiles)))
    (Variables|/Game/Tiny/Blueprints/_Core/_Game/GS_Game.GS_Game_C|SetUserProfiles _asbp_gs_game _values)))