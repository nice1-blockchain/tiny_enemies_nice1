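; Player controller for the camp-based strategy match, handling local input, camp selection and match UI.
; Clicks and a floor-projected drag box, sized on the camera pawn's CursorBox, feed same-team camps into an O_Selection object.
; Selections drive wave sends, abilities, upgrades and type resets through SRV_ events forwarded to the game state.
; OC_ events manage HUD, countdown, elimination and game-over widgets; debug keys add population and match cheats.
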(event Custom|OC_GameOver
  (params (Winner :type Integer) (StatsMatch :type S%20Stats%20Match%20Structure))
  (Utilities|FlowControl|Sequence
    (:then_0
      (if true
        (bind _wbp_eliminated (Variables|Refs|GetWBP_Eliminated)
          (:then
            (Widget|RemovefromParent _wbp_eliminated))
          (:else))))
    (:then_1
      (if true
        (Default|SetCursor (CallFunction|GetGI) "NewEnumerator5")))
    (:then_2
      (if true
        (bind _asbp_pc_game (CallFunction|GetPCGame))
        (bind _returnvalue (Team|GetTeam _asbp_pc_game))
        (if (== _returnvalue Winner)
          (Default|MusicPlay (CallFunction|GetGI) "/Game/Tiny/Art/Audio/A_MatchEnd_Succes_Cue.A_MatchEnd_Succes_Cue")
          (else
            (Default|MusicPlay (CallFunction|GetGI) "/Game/Tiny/Art/Audio/A_MatchEnd_Lose_Cue.A_MatchEnd_Lose_Cue")))))
    (:then_3
      (if true
        (bind _returnvalue_2 (UserInterface|CreateWidget "/Game/Tiny/UI/Game/Screens/WBP_GameOver.WBP_GameOver_C" 0 StatsMatch Winner))
        (bind _output_get (Variables|Refs|SetWBP_GameOver _returnvalue_2))
        (UserInterface|Viewport|AddtoViewport _output_get 50)))))

(event Custom|OC_SetTeam
  (params (Team :type Integer))
  (Variables|Team|SetTeam Team)
  (Default|SetPlayerTeam (Variables|Refs|GetWBP_GameHUD)))

(event Custom|OC_Eliminated
  (bind _returnvalue (UserInterface|CreateWidget "/Game/Tiny/UI/Game/Screens/WBP_Eliminated.WBP_Eliminated_C"))
  (bind _output_get (Variables|Refs|SetWBP_Eliminated _returnvalue))
  (UserInterface|Viewport|AddtoViewport _output_get 0))

(event Custom|SRV_Surrender
  (bind _asbp_gs_game (CallFunction|GetGSGame))
  (Default|PlayerAbandoned _asbp_gs_game self))

(event Custom|OC_RemoveCountDown
  (Utilities|FlowControl|Sequence
    (:then_0
      (Default|PreExit (Variables|Refs|GetWBP_Countdown)))
    (:then_1
      (Default|MusicPlay (CallFunction|GetGI) "/Game/Tiny/Art/Audio/A_Music_World_01.A_Music_World_01")
      (Default|SetCursor (CallFunction|GetGI) (Variables|InputCursor|GetSendPercentSelected)))))

(event Custom|SRV_CampUpgrade
  (params (CampIndex :type Integer))
  (bind _asbp_gs_game (CallFunction|GetGSGame))
  (Default|SRVCampUpgrade _asbp_gs_game self CampIndex))

(event Custom|SRV_CampAbility
  (params (CampIndex :type Integer))
  (bind _asbp_gs_game (CallFunction|GetGSGame))
  (Default|SRVCampAbility _asbp_gs_game self CampIndex))

(event Custom|SRV_WaveSpawn
  (params (Camps :type Array%20of%20Integers) (TowerEnd :type Integer) (Percent :type Integer))
  (bind _asbp_gs_game (CallFunction|GetGSGame))
  (Default|SRVWaveSpawn _asbp_gs_game self Camps TowerEnd Percent))

(event Custom|OC_StartCountdown
  (params (Seconds :type Float%20%28double-precision%29))
  (Default|LoadingScreenRemove (CallFunction|GetGI))
  (bind _returnvalue (UserInterface|CreateWidget "/Game/Tiny/UI/Game/Screens/WBP_Countdown.WBP_Countdown_C" 0 Seconds))
  (bind _output_get (Variables|Refs|SetWBP_Countdown _returnvalue))
  (UserInterface|Viewport|AddtoViewport _output_get 0))

(event Custom|OC_SetGlobalPopulation
  (params (PopulationPercents :type Array%20of%20Floats%20%28double-precision%29) (PopulationCounts :type Array%20of%20Integers))
  (bind _wbp_gamehud (Variables|Refs|GetWBP_GameHUD)
    (:then
      (Default|UpdatePopulationValues _wbp_gamehud PopulationPercents PopulationCounts))
    (:else)))

(event Custom|SRV_PCReady
  (params (UserProfile :type S%20User%20Profile%20Structure))
  (Default|CallPCReady self UserProfile))

(event Custom|OC_Widget_ProfilesCorners
  (params (UserProfiles :type Array%20of%20S%20User%20Profile%20Structures))
  (bind _wbp_gamehud (Variables|Refs|GetWBP_GameHUD)
    (:then
      (Default|UpdateProfiles _wbp_gamehud UserProfiles))
    (:else)))

(event Custom|OC_HostBackToLobby
  (Widget|RemovefromParent (Variables|Refs|GetWBP_GameHUD))
  (Default|ToLobbyEnableSwitch (Variables|Refs|GetWBP_GameOver) true))

(event Custom|SRV_CampResetTo
  (params (CampIndex :type Integer) (CampTag :type Gameplay%20Tag%20Structure))
  (bind _asbp_gs_game (CallFunction|GetGSGame))
  (Default|SRVCampResetto _asbp_gs_game self CampIndex CampTag))

(event Input|EnhancedActionEvents|EnhancedInputActionIA_Select
  (params (ActionValue :type Boolean) (ElapsedSeconds :type Float%20%28double-precision%29) (TriggeredSeconds :type Float%20%28double-precision%29) (InputAction :type Input%20Action%20Object%20Reference :default "/Game/Tiny/Data/Inputs/IA_Select.IA_Select"))
  (:Triggered
    (if (Variables|InputCursor|GetCursorLocationStartReady)
      (if (> (Math|Vector|Distance(Vector) (Variables|InputCursor|GetCursorLocationStart) (Private|MousetoFloor)) (CallFunction|GetBoxSelectionTriggerDistance))
        (Development|SetHiddeninGame (Variables|InputCursor|GetCursorBoxRef) false false)
        (bind _camps (Selection|InputBox (Private|MousetoFloor)))
        (if (Input|EnhancedActionValues|GetIA_SelectAdd)
          (Default|Add (Variables|InputCursor|GetO_Selection) _camps)
          (else
            (Default|SetFinal (Variables|InputCursor|GetO_Selection) _camps))))))
  (:Started
    (Variables|InputCursor|SetCursorLocationStart (Private|MousetoFloor))
    (Variables|InputCursor|SetCursorLocationStartReady true)
    (bind (_bisnotempty _camp _camps_2) (Selection|UnderCursorCamp))
    (if _bisnotempty
      (bind _bsameteam (Team|IsCampontheSameTeam _camps_2))
      (if _bsameteam
        (if (Input|EnhancedActionValues|GetIA_SelectAdd)
          (Default|Switch (Variables|InputCursor|GetO_Selection) _camp)
          (else
            (Default|SetFinal (Variables|InputCursor|GetO_Selection) _camp)))
        (else
          (if (not (Input|EnhancedActionValues|GetIA_SelectAdd)) :!label _label
            (Default|Clear (Variables|InputCursor|GetO_Selection)))))
      (else
        (goto _label))))
  (:Completed
    (Development|SetHiddeninGame (Variables|InputCursor|GetCursorBoxRef) true false)
    (Variables|InputCursor|SetCursorLocationStartReady false)))

(event Input|EnhancedActionEvents|EnhancedInputActionIA_Send
  (params (ActionValue :type Boolean) (ElapsedSeconds :type Float%20%28double-precision%29) (TriggeredSeconds :type Float%20%28double-precision%29) (InputAction :type Input%20Action%20Object%20Reference :default "/Game/Tiny/Data/Inputs/IA_Send.IA_Send"))
  (:Started
    (bind (_bvalid _single _camp) (Default|GetifSolo (Variables|InputCursor|GetO_Selection)))
    (bind (_bisnotempty _camp_2 _camps) (Selection|UnderCursorCamp))
    (if (Math|Boolean|ANDBoolean _bvalid _bisnotempty (== _camps _camp))
      (Default|AbilityOverlaySwitch (Variables|InputCursor|GetHoverCamp) true)
      (else
        (bind _isnotempty (Default|Get (Variables|InputCursor|GetO_Selection)))
        (if _isnotempty
          (bind (_bisnotempty_2 _camp_3 _camps_2) (Selection|UnderCursorCamp))
          (if _bisnotempty_2
            (bind _indexarray (Default|GetIndexes (Variables|InputCursor|GetO_Selection)))
            (CallFunction|SRVWaveSpawn _indexarray (Default|GetIndex _camps_2) (CallFunction|GetSendPercentValue (Variables|InputCursor|GetSendPercentSelected)))))))))

(event Input|EnhancedActionEvents|EnhancedInputActionIA_Upgrade
  (params (ActionValue :type Boolean) (ElapsedSeconds :type Float%20%28double-precision%29) (TriggeredSeconds :type Float%20%28double-precision%29) (InputAction :type Input%20Action%20Object%20Reference :default "/Game/Tiny/Data/Inputs/IA_Upgrade.IA_Upgrade"))
  (:Started
    (bind (_bvalid _single _camp) (Default|GetifSolo (Variables|InputCursor|GetO_Selection)))
    (if _bvalid
      (CallFunction|SRVCampUpgrade (Default|GetIndex _camp)))))

(event Input|EnhancedActionEvents|EnhancedInputActionIA_ResetToBarrack
  (params (ActionValue :type Boolean) (ElapsedSeconds :type Float%20%28double-precision%29) (TriggeredSeconds :type Float%20%28double-precision%29) (InputAction :type Input%20Action%20Object%20Reference :default "/Game/Tiny/Data/Inputs/IA_ResetToBarrack.IA_ResetToBarrack"))
  (bind _returnvalue (GameplayTags|MakeLiteralGameplayTag "(TagName=\"Camp.Barrack\")"))
  (:Started
    (bind (_bvalid _single _camp) (Default|GetifSolo (Variables|InputCursor|GetO_Selection)))
    (if _bvalid
      (bind _bvalid_2 (Default|HasEnough (Variables|/Game/Tiny/Blueprints/BP_Camp.BP_Camp_C|GetAC_Population _camp) (Math|Conversions|ToFloat(Integer) (.Cost (CallFunction|GetResettoValues)))))
      (if (and _bvalid_2 (!= (.type (Default|GetCampKey (Variables|/Game/Tiny/Blueprints/BP_Camp.BP_Camp_C|GetAC_State _camp))) _returnvalue))
        (CallFunction|SRVCampResetto (Default|GetIndex _camp) _returnvalue)))))

(event Input|EnhancedActionEvents|EnhancedInputActionIA_ResetToTower
  (params (ActionValue :type Boolean) (ElapsedSeconds :type Float%20%28double-precision%29) (TriggeredSeconds :type Float%20%28double-precision%29) (InputAction :type Input%20Action%20Object%20Reference :default "/Game/Tiny/Data/Inputs/IA_ResetToTower.IA_ResetToTower"))
  (bind _returnvalue (GameplayTags|MakeLiteralGameplayTag "(TagName=\"Camp.Tower\")"))
  (:Started
    (bind (_bvalid _single _camp) (Default|GetifSolo (Variables|InputCursor|GetO_Selection)))
    (if _bvalid
      (bind _bvalid_2 (Default|HasEnough (Variables|/Game/Tiny/Blueprints/BP_Camp.BP_Camp_C|GetAC_Population _camp) (Math|Conversions|ToFloat(Integer) (.Cost (CallFunction|GetResettoValues)))))
      (if (and _bvalid_2 (!= (.type (Default|GetCampKey (Variables|/Game/Tiny/Blueprints/BP_Camp.BP_Camp_C|GetAC_State _camp))) _returnvalue))
        (CallFunction|SRVCampResetto (Default|GetIndex _camp) _returnvalue)))))

(event Input|EnhancedActionEvents|EnhancedInputActionIA_ResetToWatch
  (params (ActionValue :type Boolean) (ElapsedSeconds :type Float%20%28double-precision%29) (TriggeredSeconds :type Float%20%28double-precision%29) (InputAction :type Input%20Action%20Object%20Reference :default "/Game/Tiny/Data/Inputs/IA_ResetToWatch.IA_ResetToWatch"))
  (bind _returnvalue (GameplayTags|MakeLiteralGameplayTag "(TagName=\"Camp.Watch\")"))
  (:Started
    (bind (_bvalid _single _camp) (Default|GetifSolo (Variables|InputCursor|GetO_Selection)))
    (if _bvalid
      (bind _bvalid_2 (Default|HasEnough (Variables|/Game/Tiny/Blueprints/BP_Camp.BP_Camp_C|GetAC_Population _camp) (Math|Conversions|ToFloat(Integer) (.Cost (CallFunction|GetResettoValues)))))
      (if (and _bvalid_2 (!= (.type (Default|GetCampKey (Variables|/Game/Tiny/Blueprints/BP_Camp.BP_Camp_C|GetAC_State _camp))) _returnvalue))
        (CallFunction|SRVCampResetto (Default|GetIndex _camp) _returnvalue)))))

(event Input|EnhancedActionEvents|EnhancedInputActionIA_PercentUp
  (params (ActionValue :type Boolean) (ElapsedSeconds :type Float%20%28double-precision%29) (TriggeredSeconds :type Float%20%28double-precision%29) (InputAction :type Input%20Action%20Object%20Reference :default "/Game/Tiny/Data/Inputs/IA_PercentUp.IA_PercentUp"))
  (:Started
    (Variables|InputCursor|SetSendPercentSelected (Utilities|Enum|ByteToEnumESendPercents (Math|Conversions|ToByte(Integer) (Math|Integer|Clamp(Integer) (+ (Math|Conversions|ToInteger(Byte) (Variables|InputCursor|GetSendPercentSelected)) 1) 1 (- (|GetNumEnumEntries) 1)))))
    (Default|SetCursor (CallFunction|GetGI) (Variables|InputCursor|GetSendPercentSelected))))

(event Input|EnhancedActionEvents|EnhancedInputActionIA_PercentDown
  (params (ActionValue :type Boolean) (ElapsedSeconds :type Float%20%28double-precision%29) (TriggeredSeconds :type Float%20%28double-precision%29) (InputAction :type Input%20Action%20Object%20Reference :default "/Game/Tiny/Data/Inputs/IA_PercentDown.IA_PercentDown"))
  (:Started
    (Variables|InputCursor|SetSendPercentSelected (Utilities|Enum|ByteToEnumESendPercents (Math|Conversions|ToByte(Integer) (Math|Integer|Clamp(Integer) (+ (Math|Conversions|ToInteger(Byte) (Variables|InputCursor|GetSendPercentSelected)) -1) 1 (- (|GetNumEnumEntries) 1)))))
    (Default|SetCursor (CallFunction|GetGI) (Variables|InputCursor|GetSendPercentSelected))))

(event Input|EnhancedActionEvents|EnhancedInputActionIA_Cancel
  (params (ActionValue :type Boolean) (ElapsedSeconds :type Float%20%28double-precision%29) (TriggeredSeconds :type Float%20%28double-precision%29) (InputAction :type Input%20Action%20Object%20Reference :default "/Game/Tiny/Data/Inputs/IA_Cancel.IA_Cancel"))
  (:Started
    (Default|MenuPauseSwitch (CallFunction|GetGI))))

(event Input|EnhancedActionEvents|EnhancedInputActionIA_Ability
  (params (ActionValue :type Boolean) (ElapsedSeconds :type Float%20%28double-precision%29) (TriggeredSeconds :type Float%20%28double-precision%29) (InputAction :type Input%20Action%20Object%20Reference :default "/Game/Tiny/Data/Inputs/IA_Ability.IA_Ability"))
  (:Started
    (bind (_bvalid _single _camp) (Default|GetifSolo (Variables|InputCursor|GetO_Selection)))
    (if _bvalid
      (CallFunction|SRVCampAbility (Default|GetIndex _camp)))))

(event EventTick
  (params (DeltaSeconds :type Float%20%28single-precision%29))
  (Utilities|FlowControl|Sequence
    (:then_0
      (bind (_bisnotempty _camp _camps) (Selection|UnderCursorCamp))
      (if (!= (Variables|InputCursor|GetHoverCamp) _camps)
        (bind _hovercamp (Variables|InputCursor|GetHoverCamp)
          (:then
            (Default|VisuallyOverlay _hovercamp false))
          (:else
            _))
        (if _bisnotempty
          (bind _output_get (Variables|InputCursor|SetHoverCamp _camps))
          (Default|VisuallyOverlay _output_get true)
          (else
            (Variables|InputCursor|SetHoverCamp 0)))))))

(event EventBeginPlay
  (if (Pawn|IsLocalPlayerController)
    (Utilities|FlowControl|Sequence
      (:then_0
        (if true ; PS.
          (bind _asps_game (Utilities|Casting|CastToPS_Game (Variables|GetPlayerState) :!label _label)
            (:then
              (Utilities|IsValid _asps_game
                (:Is%20Not%20Valid
                  _)))
            (:CastFailed
              _))
          (Utilities|FlowControl|Delay 0.2)
          (goto _label)))
      (:then_1
        (if true ; Hud.
          (bind _returnvalue (UserInterface|CreateWidget "/Game/Tiny/UI/Game/WBP_Game_HUD.WBP_Game_HUD_C"))
          (bind _output_get (Variables|Refs|SetWBP_GameHUD _returnvalue))
          (UserInterface|Viewport|AddtoViewport _output_get 0)))
      (:then_2
        (if true ; Input
          (Input|SetInputModeGameandUI self 0 "DoNotLock" false)
          (Class|EnhancedInputSubsystemInterface|AddPlayerMappableConfig (PlayerController|LocalPlayerSubsystems|GetEnhancedInputLocalPlayerSubsystem) "/Game/Tiny/Data/Inputs/PBIC_PlayerInputs.PBIC_PlayerInputs" "(bIgnoreAllPressedKeysUntilRelease=True,bForceImmediately=False)")))
      (:then_3
        (if true ; Selection.
          (bind _returnvalue_2 (Game|ConstructObjectfromClass "/Game/Tiny/Blueprints/_Core/_Game/O_Selection.O_Selection_C"))
          (Variables|InputCursor|SetO_Selection _returnvalue_2)))
      (:then_4
        (if true ; CursorBoxRef.
          (bind _asbp_camera_pawn (Utilities|Casting|CastToBP_Camera_Pawn (Game|Player|GetPlayerPawn 0) :!label _label_2)
            (:then
              (bind _output_get_2 (Variables|InputCursor|SetCursorBoxRef (Variables|/Game/Tiny/Blueprints/_Core/_Game/BP_Camera_Pawn.BP_Camera_Pawn_C|GetCursorBox _asbp_camera_pawn)))
              (Utilities|IsValid _output_get_2
                (:Is%20Not%20Valid
                  _)))
            (:CastFailed
              _))
          (Utilities|FlowControl|Delay 1.0)
          (Development|PrintString "Camera box ref retry.")
          (goto _label_2)))
      (:then_5
        (if true ; Ready.
          (Utilities|FlowControl|Delay 1.0)
          (CallFunction|SRVPCReady (Variables|/Game/Tiny/Blueprints/_Core/GI_Tiny.GI_Tiny_C|GetUserProfile (CallFunction|GetGI))))))))

(event EventEndPlay
  (params (EndPlayReason :type EEndPlayReason%20Enum :default "Destroyed"))
  (Default|SetCursor (CallFunction|GetGI) "NewEnumerator5"))

(event Custom|SRV_CheatInject
  (params (Indexes :type Array%20of%20Integers) (Value :type Float%20%28double-precision%29))
  (bind _asbp_gs_game (CallFunction|GetGSGame))
  (Default|ServerCheatInject _asbp_gs_game Indexes Value))

(event Input|MouseEvents|DebugKeyMiddleMouseButton
  (params (Key :type Key%20Structure) (ActionValue :type Input%20Action%20Value%20Structure))
  (:Pressed
    (if (Variables|Default|GetbCheatSwitch)
      (Utilities|IsValid (Variables|Refs|GetWBP_Debug)
        (:Is%20Valid
          (bind (_bisnotempty _camp _camps) (Selection|UnderCursorCamp))
          (if _bisnotempty
            (Default|SwitchDebugCamp (Variables|Refs|GetWBP_Debug) _camps)))))))

(event Input|KeyboardEvents|DebugKeyI
  (params (Key :type Key%20Structure) (ActionValue :type Input%20Action%20Value%20Structure))
  (:Pressed
    (if (Variables|Default|GetbCheatSwitch)
      (CallFunction|SRVCheatInject (Utilities|Array|MakeArray (Default|GetIndex (Variables|InputCursor|GetHoverCamp))) 1.0))))

(event Input|KeyboardEvents|DebugKeyP
  (params (Key :type Key%20Structure) (ActionValue :type Input%20Action%20Value%20Structure))
  (:Pressed
    (if (Variables|Default|GetbCheatSwitch)
      (if (Networking|IsServer)
        (bind _asbp_gs_game (CallFunction|GetGSGame))
        (Default|TeamEliminated _asbp_gs_game 2)))))

(event Input|KeyboardEvents|DebugKeySpaceBar
  (params (Key :type Key%20Structure) (ActionValue :type Input%20Action%20Value%20Structure))
  (:Pressed
    (bind _isa (Utilities|FlowControl|FlipFlop)
      (:A
        _)
      (:B
        _))
    (Variables|Default|SetbCheatSwitch _isa)
    (Utilities|IsValid (Variables|Refs|GetWBP_Debug)
      (:Is%20Valid
        _)
      (:Is%20Not%20Valid
        (bind _returnvalue (UserInterface|CreateWidget "/Game/Tiny/UI/_Base/Debug/WBP_Debug.WBP_Debug_C"))
        (Variables|Refs|SetWBP_Debug _returnvalue)))
    (if (Variables|Default|GetbCheatSwitch)
      (if (not (UserInterface|Viewport|IsinViewport (Variables|Refs|GetWBP_Debug)))
        (UserInterface|Viewport|AddtoViewport (Variables|Refs|GetWBP_Debug) 0))
      (else
        (Widget|RemovefromParent (Variables|Refs|GetWBP_Debug))))))

(event Input|KeyboardEvents|DebugKeyShiftI
  (params (Key :type Key%20Structure) (ActionValue :type Input%20Action%20Value%20Structure))
  (:Pressed
    (if (Variables|Default|GetbCheatSwitch)
      (CallFunction|SRVCheatInject (Utilities|Array|MakeArray (Default|GetIndex (Variables|InputCursor|GetHoverCamp))) -1.0))))

(event Input|KeyboardEvents|DebugKeyO
  (params (Key :type Key%20Structure) (ActionValue :type Input%20Action%20Value%20Structure))
  (:Pressed
    (if (Variables|Default|GetbCheatSwitch)
      (if (Networking|IsServer)
        (bind _asbp_gs_game (CallFunction|GetGSGame))
        (Default|SRVGameOver _asbp_gs_game 1)))))

(event Input|KeyboardEvents|DebugKeyShift5
  (params (Key :type Key%20Structure) (ActionValue :type Input%20Action%20Value%20Structure))
  (:Pressed
    (if (Variables|Default|GetbCheatSwitch)
      (CallFunction|SRVCheatInject (Utilities|Array|MakeArray (Default|GetIndex (Variables|InputCursor|GetHoverCamp))) -5e+01))))

(event Input|KeyboardEvents|DebugKey5
  (params (Key :type Key%20Structure) (ActionValue :type Input%20Action%20Value%20Structure))
  (:Pressed
    (if (Variables|Default|GetbCheatSwitch)
      (CallFunction|SRVCheatInject (Utilities|Array|MakeArray (Default|GetIndex (Variables|InputCursor|GetHoverCamp))) 5e+01))))

(fn ConstructionScript
  (|CallParentFunction))

(fn MousetoFloor
  (bind (_locationx _locationy) (Game|Player|GetMousePosition))
  (bind (_worldlocation _worlddirection) (Class|PlayerController|DeprojectScreenPositiontoWorld _locationx _locationy))
  (return (.Intersection (Class|KismetMathLibrary|LinePlaneIntersectionOriginNormal _worldlocation (+ _worldlocation (* _worlddirection 3e+04)) "0, 0, 0" "0,0.000000,1.000000"))))

(fn UnderCursorCamp
  (bind _asbp_camp (Utilities|Casting|CastToBP_Camp (.HitActor (Collision|BreakHitResult (.HitResult (Class|PlayerController|GetHitResultUnderCursorforObjects (Utilities|Array|MakeArray "ObjectTypeQuery7") false)))))
    (:then
      (return (Utilities|Set|IsNotEmpty (Utilities|Set|MakeSet _asbp_camp)) (Utilities|Set|MakeSet _asbp_camp) _asbp_camp))
    (:CastFailed
      (return false 0 0))))

(fn InputBox
  (params (CursorLocationCurrent :type Vector))
  (bind _returnvalue (Math|Float|MakeLiteralFloat 0.5))
  (bind _cursorlocationstart (Variables|InputCursor|GetCursorLocationStart))
  (bind _cursorlocationstart_2 (Variables|InputCursor|GetCursorLocationStart))
  (bind _returnvalue_2 (- CursorLocationCurrent _cursorlocationstart_2))
  (bind _returnvalue_3 (+ CursorLocationCurrent _cursorlocationstart))
  (bind _returnvalue_4 (* _returnvalue_3 0.5))
  (Transformation|SetWorldScale3D (Variables|InputCursor|GetCursorBoxRef) (Math|Vector|MakeVector (* (Math|Vector|VectorLength (Math|Vector|ProjectVectorontoVector _returnvalue_2 "1.000000, 0, 0")) _returnvalue) (* (Math|Vector|VectorLength (Math|Vector|ProjectVectorontoVector _returnvalue_2 "0,1.000000, 0")) _returnvalue) 2e+01))
  (Transformation|SetWorldLocation (Variables|InputCursor|GetCursorBoxRef) _returnvalue_4 false false)
  (bind _outactors (Collision|ComponentOverlapActors (Variables|InputCursor|GetCursorBoxRef) (Math|Transform|MakeTransform _returnvalue_4 "0, 0, 0" "1.000000,1.000000,1.000000") (Utilities|Array|MakeArray "ObjectTypeQuery8") "/Game/Tiny/Blueprints/BP_Camp.BP_Camp_C"))
  (for _array_element _outactors
    (bind _asbp_camp (Utilities|Casting|CastToBP_Camp _array_element))
    (bind _bsameteam (Team|IsCampontheSameTeam _asbp_camp))
    (if _bsameteam
      (Utilities|Set|Add (LocalVariables|Get_Camps) _asbp_camp)))
  (return (LocalVariables|Get_Camps)))

(fn IsCampontheSameTeam
  (params (Camp :type BP%20Camp%20Object%20Reference))
  (return (== (Default|GetTeamValue (Variables|/Game/Tiny/Blueprints/BP_Camp.BP_Camp_C|GetAC_Team Camp)) (Variables|Team|GetTeam))))

(fn GetTeam
  (return (Variables|Team|GetTeam)))