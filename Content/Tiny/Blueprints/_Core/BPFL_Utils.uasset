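; Blueprint function library of shared helpers for screen popups and depth sorting.
; ScreenConfirmation and ScreenLoading create confirmation and match-loading widgets for the local player controller at index 0, add them to the viewport and return them.
; The confirmation takes custom text and an alternate-button switch, and uses a high Z-order to sit on top.
; UpdateZOrder fakes draw order by remapping a component's world Y, unclamped, into its world Z.
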(fn ScreenConfirmation
  (params (Message :type Text) (TextLeft :type Text) (RightButtonSwitch :type Boolean) (TextRight :type Text))
  (bind _returnvalue (Game|GetPlayerController 0))
  (if (Pawn|IsLocalPlayerController _returnvalue)
    (bind _returnvalue_2 (UserInterface|CreateWidget "/Game/Tiny/UI/Menu/Screens/WBP_ScreenConfirmation.WBP_ScreenConfirmation_C" _returnvalue Message TextLeft TextRight RightButtonSwitch))
    (UserInterface|Viewport|AddtoViewport _returnvalue_2 1000)
    (return _returnvalue_2)))

(fn ScreenLoading
  (bind _returnvalue (Game|GetPlayerController 0))
  (if (Pawn|IsLocalPlayerController _returnvalue)
    (bind _returnvalue_2 (UserInterface|CreateWidget "/Game/Tiny/UI/Game/Screens/WBP_LoadingMatch.WBP_LoadingMatch_C" _returnvalue))
    (UserInterface|Viewport|AddtoViewport _returnvalue_2 0)
    (return _returnvalue_2)))

(fn UpdateZOrder
  (params (Component :type Scene%20Component%20Object%20Reference))
  (bind _returnvalue (Transformation|GetWorldLocation Component))
  (Transformation|SetWorldLocation Component (Math|Vector|MakeVector (.x _returnvalue) (.y _returnvalue) (Math|Float|MapRangeUnclamped (.y _returnvalue) -2e+03 2e+03 0.0 1e+02)) false false)
  (return))