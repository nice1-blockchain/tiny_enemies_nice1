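; Lobby game mode that tracks connected players and launches the game world for everyone.
; It keeps a list of player controllers, updated on login, controller swap and logout, and also removes leaving players from the lobby game state.
; On launch it clears each lobby controller's widgets, then server-travels to the map resolved from the game state's selected world enum via a soft reference.
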(event Custom|LaunchGameWorld
  (Utilities|FlowControl|Sequence
    (:then_0
      (for _array_element (Variables|Default|GetAll_PC's)
        (bind _aspc_lobby (Utilities|Casting|CastToPC_Lobby _array_element))
        (Default|RemoveWidgets _aspc_lobby)))
    (:then_1
      (bind _worldsoft (CallFunction|GetWorldEnumtoSoft (Default|GetCurrentWorld (CallFunction|GetGSLobby))))
      (Private|ServerTraveltoMap _worldsoft))))

(event EventPostLogin
  (params (NewPlayer :type Player%20Controller%20Object%20Reference))
  (CallFunction|PlayerConnect NewPlayer))

(event EventOnSwapPlayerControllers
  (params (OldPC :type Player%20Controller%20Object%20Reference) (NewPC :type Player%20Controller%20Object%20Reference))
  (CallFunction|PlayerConnect NewPC))

(event EventOnLogout
  (params (ExitingController :type Controller%20Object%20Reference))
  (bind _asplayer_controller (Utilities|Casting|CastToPlayerController ExitingController))
  (CallFunction|PlayerDisconnect _asplayer_controller)
  (Default|RemovePlayer (CallFunction|GetGSLobby) _asplayer_controller))

(fn ConstructionScript)

(fn PlayerConnect
  (params (NewPlayer :type Player%20Controller%20Object%20Reference))
  (Utilities|Array|Add (Variables|Default|GetAll_PC's) NewPlayer))

(fn PlayerDisconnect
  (params (PC :type Player%20Controller%20Object%20Reference%20%28by%20ref%29))
  (Utilities|Array|RemoveItem (Variables|Default|GetAll_PC's) PC)
  (return))

(fn ServerTraveltoMap
  (params (Level :type World%20Soft%20Object%20Reference))
  (bind _returnvalue (Class|AdvancedSessionsLibrary|ServerTravel (Class|BlueprintPathsLibrary|GetBaseFilename (Utilities|ToString(SoftObjectReference) Level) true) true false))
  (if _returnvalue
    (Development|PrintString "Launching game... ")
    (else
      (Development|PrintString "Server travel fail."))))