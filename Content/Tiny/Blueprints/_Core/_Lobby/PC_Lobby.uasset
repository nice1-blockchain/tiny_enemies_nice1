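; Lobby player controller that owns the local lobby UI and relays player data between the client and the lobby game state.
; On BeginPlay the local controller shows the lobby widget, polls until its unique net ID is valid, then sends the user profile and connection info through SRV_AddPlayer.
; SRV events register the player and ready state, OC events refresh the widget's player list and world, and other events handle loading-screen creation and widget removal.
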(event Custom|LoadingScreen
  (bind _returnvalue (UserInterface|CreateWidget "/Game/Tiny/UI/Menu/Screens/WBP_ScreenLoading.WBP_ScreenLoading_C"))
  (UserInterface|Viewport|AddtoViewport _returnvalue 0)
  (Variables|Default|SetWBP_LoadingScreen _returnvalue))

(event Custom|OC_UpdatePlayerList
  (params (ConnectedUsers :type Array%20of%20S%20Connected%20User%20Structures))
  (Default|UpdatePlayerList (Variables|Default|GetWBP_Lobby) ConnectedUsers))

(event Custom|OC_UpdateCurrentWorld
  (params (World :type Gameplay%20Tag%20Structure))
  (Default|UpdateWorld (Variables|Default|GetWBP_Lobby) World))

(event Custom|SRV_AddPlayer
  (params (ConnectedUser :type S%20Connected%20User%20Structure))
  (Default|AddPlayerProfile (CallFunction|GetGSLobby) self ConnectedUser))

(event Custom|RemoveWidgets
  (Widget|RemovefromParent (Variables|Default|GetWBP_Lobby))
  (Widget|RemovefromParent (Variables|Default|GetWBP_LoadingScreen)))

(event Custom|SRV_SetReadyStateFromLobby
  (params (IsReady :type Boolean))
  (Default|PlayerReady (CallFunction|GetGSLobby) self IsReady))

(event EventBeginPlay
  (bind _self self)
  (bind _uniquenetid (Class|AdvancedSessionsLibrary|GetUniqueNetID _self))
  (if (Pawn|IsLocalPlayerController)
    (Utilities|FlowControl|Sequence
      (:then_0
        (if true
          (bind _returnvalue (UserInterface|CreateWidget "/Game/Tiny/UI/Menu/WBP_Lobby.WBP_Lobby_C"))
          (bind _output_get (Variables|Default|SetWBP_Lobby _returnvalue))
          (UserInterface|Viewport|AddtoViewport _output_get 0)))
      (:then_1
        (if true ; Send UserProfile to SRV_GS
          (if (Class|AdvancedSessionsLibrary|IsValidUniqueNetID _uniquenetid) :!label _label
            (CallFunction|SRVAddPlayer (Utilities|Struct|MakeSConnectedUser (Variables|/Game/Tiny/Blueprints/_Core/GI_Tiny.GI_Tiny_C|GetUserProfile (CallFunction|GetGI)) (Utilities|Struct|MakeSConnectInfo (Class|AdvancedSessionsLibrary|UniqueNetIdtoString _uniquenetid) (Networking|IsServer) false)))
            (else
              (Utilities|FlowControl|Delay 0.2)
              (goto _label))))))))

(fn ConstructionScript)

(fn IsMeUniqueNetID
  (params (UniqueNetID :type String))
  (return (Utilities|Enum|Equal(Enum) UniqueNetID (Class|AdvancedSessionsLibrary|UniqueNetIdtoString (Class|AdvancedSessionsLibrary|GetUniqueNetID self)))))