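; Global function library that centralizes tuning constants for a team-based game of camps sending unit waves.
; Hardcoded getters cover wave movement and formation, shooting, growth, costs and timings, box selection, save slot names and loading time.
; Lookup helpers map teams to colors, send percentages to values, map names to world tags (defaulting to W1), and tags to world assets.
; The asset lookup has no entry for W7.
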(fn GetUserProfileSlot
  (return "UserProfileSlot"))

(fn GetCampGoalRadius
  (return 5.0))

(fn GetStartCountdown
  (return 1.0))

(fn GetCommandCooldown
  (return 0.5))

(fn GetWaveSpeed
  (return 225.0))

(fn GetWavetoCampTransferSpeed
  (return 0.15 1.0))

(fn GetWaveSendMin
  (return 1))

(fn GetSoundProfileSlot
  (return "SoundProfileSlot"))

(fn GetLoadingScreenTime
  (return 4.0))

(fn GetTeamColor
  (params (Team :type Integer))
  (return (Utilities|Select :Index Team :Option%200 "(R=0.321875,G=0.321875,B=0.321875,A=1.000000)" :Option%201 "(R=0.106988,G=0.264298,B=0.708333,A=1.000000)" :Option%202 "(R=0.127019,G=0.546875,B=0.122477,A=1.000000)" :Option%203 "(R=0.496875,G=0.188916,B=0.430225,A=1.000000)" :Option%204 "(R=0.467709,G=0.329176,B=0.252855,A=1.000000)")))

(fn GetWaveSendMax
  (return 10000))

(fn GetSendPercentValue
  (params (SpawnPercent :type ESendPercents%20Enum :default "NewEnumerator0"))
  (return (Utilities|Select :Index SpawnPercent :NewEnumerator1 25 :NewEnumerator2 50 :NewEnumerator3 75 :NewEnumerator4 100)))

(fn GetShootEnable
  (return true))

(fn GetGrowEnable
  ;[1 1 1] Unused
  (return false))

(fn GetGrowCadence
  (return 1.0))

(fn GetGrowNeutralValues
  (return 0.5 1.5 3.0))

(fn GetShootProjectileTravelTime
  (return 0.4))

(fn GetWaveRowSeparation
  (return 0.3))

(fn GetWaveRowUnitSeparation
  (return 45.0))

(fn GetWaveRowUnitsMax
  (return 10))

(fn GetResettoValues
  (return 20 5.0))

(fn GetObserverValues
  (return 1 3.0 1125.0))

(fn GetCampDowngradeValues
  (return 0.5))

(fn GetWorldEnumtoSoft
  (params (World :type Gameplay%20Tag%20Structure))
  (Utilities|FlowControl|Sequence
    (:then_0
      (|SwitchGameplayTag World
        (:World.W1
          (LocalVariables|SetIndex 1))
        (:World.W2
          (LocalVariables|SetIndex 2))
        (:World.W3
          (LocalVariables|SetIndex 3))
        (:World.W4
          (LocalVariables|SetIndex 4))
        (:World.W5
          (LocalVariables|SetIndex 5))
        (:World.W6
          (LocalVariables|SetIndex 6))
        (:World.W7
          (LocalVariables|SetIndex 7))))
    (:then_1
      (return (Utilities|Select :Index (LocalVariables|GetIndex) :Option%200 0 :Option%201 "/Game/Tiny/Maps/Worlds/World_01.World_01" :Option%202 "/Game/Tiny/Maps/Worlds/World_02.World_02" :Option%203 "/Game/Tiny/Maps/Worlds/World_03.World_03" :Option%204 "/Game/Tiny/Maps/Worlds/World_04.World_04" :Option%205 "/Game/Tiny/Maps/Worlds/World_05.World_05" :Option%206 "/Game/Tiny/Maps/Worlds/World_06.World_06")))))

(fn GetWorldTagfromMapName
  (params (MapName :type String))
  (switch string MapName
    (:Default
      _)
    (:World_01
      _)
    (:World_02
      (return "(TagName=\"World.W2\")"))
    (:World_03
      (return "(TagName=\"World.W3\")"))
    (:World_04
      (return "(TagName=\"World.W4\")"))
    (:World_05
      (return "(TagName=\"World.W5\")"))
    (:World_06
      (return "(TagName=\"World.W6\")"))
    (:World_07
      (return "(TagName=\"World.W7\")")))
  (return "(TagName=\"World.W1\")"))

(fn GetBoxSelectionTriggerDistance
  (return 25.0))

(fn GetYScaletoMatchPerspective
  (return 0.7))