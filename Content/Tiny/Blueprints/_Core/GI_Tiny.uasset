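; Game instance for Tiny that holds game-wide services: settings, profiles, audio, shared UI and error reporting.
; Init loads user settings and save-slot user and sound profiles, creating defaults when loading fails, then applies volumes through a sound mix.
; It keeps music playing across level transitions and manages loading-screen and pause-menu widgets.
; Network and travel failures are stored as strings until DispatchErrors shows them in a confirmation screen.
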(event Custom|ApplySoundProfile
  (params (SSoundProfile :type S%20Sound%20Profile%20Structure%20%28by%20ref%29))
  (bind (_musicvolume _effectsvolume) (Utilities|Struct|BreakSSoundProfile SSoundProfile))
  (Utilities|FlowControl|Sequence
    (:then_0
      (Audio|SetSoundMixClassOverride "/Game/Tiny/Art/Audio/Class/SCM_MasterSound.SCM_MasterSound" "/Game/Tiny/Art/Audio/Class/SC_Music.SC_Music" _musicvolume 1.0 0.0 true)
      (Audio|PushSoundMixModifier "/Game/Tiny/Art/Audio/Class/SCM_MasterSound.SCM_MasterSound"))
    (:then_1
      (Audio|SetSoundMixClassOverride "/Game/Tiny/Art/Audio/Class/SCM_MasterSound.SCM_MasterSound" "/Game/Tiny/Art/Audio/Class/SC_Effects.SC_Effects" _effectsvolume 1.0 0.0 true)
      (Audio|PushSoundMixModifier "/Game/Tiny/Art/Audio/Class/SCM_MasterSound.SCM_MasterSound"))))

(event Custom|MusicPlay
  (params (Sound :type Sound%20Base%20Object%20Reference))
  (Utilities|FlowControl|Delay 0.2)
  (Utilities|IsValid (Variables|Default|GetMusic)
    (:Is%20Valid
      (if (!= (Variables|/Script/Engine.AudioComponent|GetSound (Variables|Default|GetMusic)) Sound)
        (Audio|Components|Audio|SetSound (Variables|Default|GetMusic) Sound)
        (Audio|Components|Audio|Play (Variables|Default|GetMusic) 0.0)))
    (:Is%20Not%20Valid
      (bind _returnvalue (Audio|CreateSound2D Sound 1.0 1.0 0.0 0 true))
      (bind _output_get (Variables|Default|SetMusic _returnvalue))
      (Audio|Components|Audio|Play _output_get 0.0))))

(event Custom|LoadingScreenStart
  (params (ConnectedUsers :type Array%20of%20S%20Connected%20User%20Structures) (CurrentWorld :type Gameplay%20Tag%20Structure))
  (bind _returnvalue (UserInterface|CreateWidget "/Game/Tiny/UI/Game/Screens/WBP_LoadingMatch.WBP_LoadingMatch_C" 0 ConnectedUsers CurrentWorld))
  (UserInterface|Viewport|AddtoViewport _returnvalue 100)
  (Variables|Default|SetWBP_LoadingScreen _returnvalue))

(event Custom|LoadingScreenRemove
  (bind _wbp_loadingscreen (Variables|Default|GetWBP_LoadingScreen))
  (Utilities|IsValid _wbp_loadingscreen
    (:Is%20Valid
      (Widget|RemovefromParent _wbp_loadingscreen))))

(event Custom|MusicStop
  (Utilities|IsValid (Variables|Default|GetMusic)
    (:Is%20Valid
      (Audio|Components|Audio|Stop (Variables|Default|GetMusic)))))

(event Custom|QuitGame
  (Game|QuitGame 0 "Quit" false))

(event EventInit
  (|CallParentFunction)
  (Utilities|FlowControl|Sequence
    (:then_0
      (bind _returnvalue (Settings|GetGameUserSettings))
      (Class|GameUserSettings|ValidateSettings _returnvalue)
      (Class|GameUserSettings|LoadSettings _returnvalue true))
    (:then_1
      (if true ; UserProfile
        (bind _valid (UserProfile|UserProfileLoad))
        (if (not _valid)
          (Variables|Profiles|SetUserProfile (Utilities|Struct|MakeSUserProfile "Username" "/Game/Tiny/Art/UI/Avatar/T_Avatar_Baby.T_Avatar_Baby"))
          (UserProfile|UserProfileSave))))
    (:then_2
      (if true ; SoundProfile
        (bind _valid_2 (SoundProfile|SoundProfileLoad))
        (if (not _valid_2)
          (Variables|Profiles|SetSoundProfile (Utilities|Struct|MakeSSoundProfile 1.0 1.0))
          (SoundProfile|SoundProfileSave))
        (Utilities|FlowControl|Delay 0.2)
        (CallFunction|ApplySoundProfile (Variables|Profiles|GetSoundProfile))))))

(event EventHandleTravelError
  (params (FailureType :type ETravelFailure%20Enum :default "NoLevel"))
  (Variables|ErrorHandle|SetTravelError (Utilities|String|EnumtoString FailureType)))

(event EventHandleNetworkError
  (params (FailureType :type ENetworkFailure%20Enum :default "NetDriverAlreadyExists") (bIsServer :type Boolean))
  (Variables|ErrorHandle|SetNetworkError (Utilities|String|EnumtoString FailureType)))

(fn UserProfileSave
  (bind _returnvalue (SaveGame|CreateSaveGameObject "/Game/Tiny/Blueprints/_Core/Structures/SG_UserProfile.SG_UserProfile_C"))
  (bind _output_get (LocalVariables|SetSaveGameObject _returnvalue))
  (Variables|/Game/Tiny/Blueprints/_Core/Structures/SG_UserProfile.SG_UserProfile_C|SetSUserProfile _output_get (Variables|Profiles|GetUserProfile))
  (bind _returnvalue_2 (SaveGame|SaveGametoSlot (LocalVariables|GetSaveGameObject) (CallFunction|GetUserProfileSlot)))
  (return _returnvalue_2))

(fn UserProfileLoad
  (bind _returnvalue (SaveGame|DoesSaveGameExist (CallFunction|GetUserProfileSlot)))
  (if _returnvalue
    (bind _returnvalue_2 (SaveGame|LoadGamefromSlot (CallFunction|GetUserProfileSlot)))
    (bind _assg_user_profile (Utilities|Casting|CastToSG_UserProfile _returnvalue_2)
      (:then
        (Variables|Profiles|SetUserProfile (Variables|/Game/Tiny/Blueprints/_Core/Structures/SG_UserProfile.SG_UserProfile_C|GetSUserProfile _assg_user_profile))
        (return true))
      (:CastFailed
        _)))
  (return false))

(fn IsSessionValid
  (params (Session :type Blueprint%20Session%20Result%20Structure))
  (return (> (Class|FindSessionsCallbackProxy|GetCurrentPlayers Session) 0)))

(fn MenuPauseSwitch
  (bind _wbp_pausemenu (Variables|Menu|GetWBP_PauseMenu)
    (:then
      (if (UserInterface|Viewport|IsinViewport _wbp_pausemenu)
        (Default|EscapeRoute (Variables|Menu|GetWBP_PauseMenu))
        (else
          (UserInterface|Viewport|AddtoViewport (Variables|Menu|GetWBP_PauseMenu) 100 :!label _label))))
    (:else
      (bind _returnvalue (UserInterface|CreateWidget "/Game/Tiny/UI/Game/Screens/WBP_Pause.WBP_Pause_C"))
      (Variables|Menu|SetWBP_PauseMenu _returnvalue)
      (goto _label))))

(fn DispatchErrors
  (bind _gi (CallFunction|GetGI))
  (bind _gi_2 (CallFunction|GetGI))
  (if (and (Utilities|Array|IsEmpty (Variables|ErrorHandle|GetNetworkError)) (Utilities|Array|IsEmpty (Variables|ErrorHandle|GetTravelError)))
    (return)
    (else
      (Utilities|FlowControl|Sequence
        (:then_0
          (if (not (Utilities|Array|IsEmpty (Variables|GI_Tiny_C|GetNetworkError _gi_2)))
            (CallFunction|ScreenConfirmation (Utilities|Text|ToText(String) (Utilities|String|Append "Error: " (Variables|GI_Tiny_C|GetNetworkError _gi_2))) "Ok" false)
            (Variables|GI_Tiny_C|SetNetworkError _gi_2 "")
            (return)))
        (:then_1
          (if (not (Utilities|Array|IsEmpty (Variables|GI_Tiny_C|GetTravelError _gi)))
            (CallFunction|ScreenConfirmation (Utilities|Text|ToText(String) (Utilities|String|Append "Error: " (Variables|GI_Tiny_C|GetTravelError _gi))) "Ok" false)
            (Variables|GI_Tiny_C|SetTravelError _gi "")
            (return)))))))

(fn SoundProfileSave
  (bind _returnvalue (SaveGame|CreateSaveGameObject "/Game/Tiny/Blueprints/_Core/Structures/SG_SoundProfile.SG_SoundProfile_C"))
  (bind _output_get (LocalVariables|Set_SaveGameObject _returnvalue))
  (Variables|/Game/Tiny/Blueprints/_Core/Structures/SG_SoundProfile.SG_SoundProfile_C|SetSSoundProfile _output_get (Variables|Profiles|GetSoundProfile))
  (bind _returnvalue_2 (SaveGame|SaveGametoSlot (LocalVariables|Get_SaveGameObject) (CallFunction|GetSoundProfileSlot)))
  (return _returnvalue_2))

(fn SoundProfileLoad
  (bind _returnvalue (SaveGame|DoesSaveGameExist (CallFunction|GetSoundProfileSlot)))
  (if _returnvalue
    (bind _returnvalue_2 (SaveGame|LoadGamefromSlot (CallFunction|GetSoundProfileSlot)))
    (bind _assg_sound_profile (Utilities|Casting|CastToSG_SoundProfile _returnvalue_2)
      (:then
        (Variables|Profiles|SetSoundProfile (Variables|/Game/Tiny/Blueprints/_Core/Structures/SG_SoundProfile.SG_SoundProfile_C|GetSSoundProfile _assg_sound_profile))
        (return true))
      (:CastFailed
        (return false)))
    (else
      (return false))))