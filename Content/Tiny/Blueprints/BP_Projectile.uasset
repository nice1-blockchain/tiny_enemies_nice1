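; Projectile actor that homes in on a target BPUnit and delivers a hit on arrival.
; A timeline, with play rate scaled to the shot's travel time, lerps it from its spawn point to the target flipbook's current location.
; When the timeline finishes, it destroys itself and calls the hit on the unit if still valid.
; If the target is lost mid-flight, it destroys itself early.
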(event EventBeginPlay
  (Variables|Default|SetStartingLocation (Transformation|GetWorldLocation (Variables|Default|GetRoot)))
  (Components|Timeline|SetPlayRate (Variables|Default|GetTrajectoryTimeline) (/ 1.0 (CallFunction|GetShootProjectileTravelTime)))
  (bind _trajectory (Timeline|TrajectoryTimeline Play)
    (:Update
      (Utilities|IsValid (Variables|Default|GetBP_Unit)
        (:Is%20Valid
          (if (not (Game|IsActorBeingDestroyed (Variables|Default|GetBP_Unit)))
            (Transformation|SetWorldLocation (Variables|Default|GetRoot) (Math|Vector|Lerp(Vector) (Variables|Default|GetStartingLocation) (Transformation|GetWorldLocation (Variables|/Game/Tiny/Blueprints/BP_Unit.BP_Unit_C|GetPaperFlipbook (Variables|Default|GetBP_Unit))) _trajectory) false false)
            (else
              (Actor|DestroyActor :!label _label)
              (Utilities|IsValid (Variables|Default|GetBP_Unit)
                (:Is%20Valid
                  (if (not (Game|IsActorBeingDestroyed (Variables|Default|GetBP_Unit)))
                    (Default|CallHit (Variables|Default|GetBP_Unit))))))))
        (:Is%20Not%20Valid
          (goto _label))))
    (:Finished
      (goto _label))))

(fn ConstructionScript)