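; BP_Camp is a capturable, team-owned House, Tower or Forge whose population pays for timed upgrades and type resets.
; Team, Population and Upgrade components are server-initialised, with update events bound for sprite and overlay visuals.
; Houses get grow components (neutral variant for team 0) and Towers sensing-sphere shooters, created at runtime and removed during construction.
; Income drains population scaled by attack and defense; depletion switches team, triggers downgrade and injects leftover attackers.
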(event Custom|Construct
  (Components|CampTypeComponentsAdd))

(event Custom|SetDecalSwitch
  (params (bNewVisibility :type Boolean))
  (Rendering|SetVisibility (Variables|Default|GetDecal) bNewVisibility false))

(event Custom|UpgradeFinished
  (Utilities|Time|ClearandInvalidateTimerbyHandle (stale Custom|Upgrade _returnvalue_3))
  (Default|SetLevel (Variables|Default|GetAC_Upgrade) false)
  (Components|CampTypeComponentsAdd)
  (Default|SetRunState (Variables|Default|GetAC_Upgrade) "NewEnumerator1"))

(event Custom|SetUpgradeOverlay
  (params (bSwitch :type Boolean))
  (Default|SetSwitch (Variables|Refs|GetWBP_UpgradeOverlay) bSwitch))

(event Custom|Downgrade
  (bind _bvalid (Default|CanbeDowngraded (Variables|Default|GetAC_Upgrade)))
  (if _bvalid
    (bind _returnvalue (Utilities|Time|SetTimerbyEvent (delegate Custom|DowngradeFinished) (CallFunction|GetCampDowngradeTime)))
    (Components|CampTypeComponentsRemove)
    (Default|SetRunState (Variables|Default|GetAC_Upgrade) "NewEnumerator2")
    (elif true ; Reset.
      (Components|CampTypeComponentsRemove)
      (Components|CampTypeComponentsAdd))))

(event Custom|Upgrade
  (bind _ac_upgrade (Variables|Default|GetAC_Upgrade))
  (bind _returnvalue (Default|GetUpgrade _ac_upgrade))
  (bind _returnvalue_2 (Math|Conversions|ToFloat(Integer) (.nextcost _returnvalue)))
  (bind _bvalid (Default|CanbeUpgraded (Variables|Default|GetAC_Upgrade)))
  (if _bvalid
    (bind _bvalid_2 (Default|HasEnough (Variables|Default|GetAC_Population) _returnvalue_2))
    (if _bvalid_2
      (Default|Extract (Variables|Default|GetAC_Population) _returnvalue_2)
      (bind _returnvalue_3 (Utilities|Time|SetTimerbyEvent (delegate Custom|UpgradeFinished) (.nexttime _returnvalue)))
      (Components|CampTypeComponentsRemove)
      (Default|SetRunState (Variables|Default|GetAC_Upgrade) "NewEnumerator2"))))

(event Custom|HitFX
  (params (Unit :type BP%20Unit%20Object%20Reference))
  (Audio|PlaySound2D 0 1.0 1.0 0.0 0 0)
  (Utilities|IsValid Unit
    (:Is%20Valid
      (Actor|DestroyActor Unit))))

(event Custom|ResetFinish
  (Utilities|Time|ClearandInvalidateTimerbyHandle (stale Custom|ResetTo _returnvalue_2))
  (Default|SetResetto (Variables|Default|GetAC_Upgrade) (stale Custom|ResetTo Camp))
  (Components|CampTypeComponentsAdd)
  (Default|SetRunState (Variables|Default|GetAC_Upgrade) "NewEnumerator1"))

(event Custom|ResetTo
  (params (Camp :type Gameplay%20Tag%20Structure))
  (bind (_time _count) (CallFunction|GetCampResetCost))
  (bind _returnvalue (Math|Conversions|ToFloat(Integer) _count))
  (bind _bvalid (Default|HasEnough (Variables|Default|GetAC_Population) _returnvalue))
  (if _bvalid
    (Default|Extract (Variables|Default|GetAC_Population) _returnvalue)
    (bind _returnvalue_2 (Utilities|Time|SetTimerbyEvent (delegate Custom|ResetFinish) _time))
    (Components|CampTypeComponentsRemove)
    (Default|SetRunState (Variables|Default|GetAC_Upgrade) "NewEnumerator2")))

(event Custom|DowngradeFinished
  (Utilities|Time|ClearandInvalidateTimerbyHandle (stale Custom|Downgrade _returnvalue))
  (Default|SetLevel (Variables|Default|GetAC_Upgrade) true)
  (Components|CampTypeComponentsAdd)
  (Default|SetRunState (Variables|Default|GetAC_Upgrade) "NewEnumerator1"))

(event Custom|Income
  (params (Team :type Integer) (Value :type Float%20%28double-precision%29) (AtackMultiplier :type Float%20%28double-precision%29))
  (bind _returnvalue (Actor|GetComponentbyClass "/Game/Tiny/Blueprints/Components/AC_GrowNeutral.AC_GrowNeutral_C"))
  (Utilities|FlowControl|Sequence
    (:then_0
      (bind (_bdepleted _extracted) (Default|Extract (Variables|Default|GetAC_Population) (/ (* AtackMultiplier Value) (.Defense (Utilities|Struct|BreakSUpgrade (Default|GetUpgrade (Variables|Default|GetAC_Upgrade)))))))
      (if _bdepleted
        (Default|SetTeamValue (Variables|Default|GetAC_Team) Team)
        (CallFunction|Downgrade)
        (Default|Inject (Variables|Default|GetAC_Population) (- Value _extracted))))
    (:then_1
      (if true ; Last atack timer for neutral grow.
        (Utilities|IsValid _returnvalue
          (:Is%20Valid
            (Default|SetGrowStartDelay _returnvalue)))))))

(event Custom|ShootFX
  (params (Unit :type BP%20Unit%20Object%20Reference))
  (Utilities|IsValid Unit
    (:Is%20Valid
      (Sprite|SetSpriteColor (Variables|/Game/Tiny/Blueprints/BP_Unit.BP_Unit_C|GetPaperFlipbook Unit) "(R=1.000000,G=0.000000,B=0.000000,A=1.000000)")
      (bind _returnvalue (Game|SpawnActorfromClass "/Game/Tiny/Blueprints/BP_Projectile.BP_Projectile_C" (Transformation|GetWorldTransform (Variables|Default|GetFiringSpot)) "Undefined" 0 Unit 0))
      (EventDispatchers|BindEventtoHit _returnvalue (EventDispatchers|CreateEvent :!event Custom|HitFX)))
    (:Is%20Not%20Valid
      (Development|PrintString "BP_Camp/ShootFX/Not valid unit"))))

(event Custom|InitialVisualValues
  (bind _initialcamp (Variables|InitialExposedValues|GetInitialCamp))
  (Visual|VisualSetTypeandLevel (.type _initialcamp) (.level _initialcamp) "NewEnumerator0")
  (Visual|VisualSetTeam (Variables|InitialExposedValues|GetInitialTeam)))

(event EventBeginPlay
  (bind _initialcamp (Variables|InitialExposedValues|GetInitialCamp))
  (Utilities|FlowControl|Sequence
    (:then_0
      (if true ; Add PopulationOverlay.
        (bind _returnvalue (AddComponent|AddWidgetComponent false))
        (bind _aswbp_camp_overlay (Utilities|Casting|CastToWBP_CampOverlay (UserInterface|GetWidget _returnvalue)))
        (Variables|Refs|SetWBP_CampOverlay _aswbp_camp_overlay)))
    (:then_1
      (if true ; Add UpgradeOverlay.
        (bind _returnvalue_2 (AddComponent|AddWidgetComponent false))
        (bind _aswbp_upgrade_overlay (Utilities|Casting|CastToWBP_UpgradeOverlay (UserInterface|GetWidget _returnvalue_2)))
        (Variables|Refs|SetWBP_UpgradeOverlay _aswbp_upgrade_overlay)))
    (:then_2
      (if true ; Team Bind/Set
        (EventDispatchers|BindEventtoTeamUpdated (Variables|Default|GetAC_Team) (EventDispatchers|CreateEvent :!event VisualSetTeam))
        (if (Networking|IsServer)
          (Default|SetTeamValue (Variables|Default|GetAC_Team) (Variables|InitialExposedValues|GetInitialTeam))
          (else
            (Visual|VisualSetTeam (Variables|InitialExposedValues|GetInitialTeam))))))
    (:then_3
      (if true ; Population Bind/Set
        (EventDispatchers|BindEventtoPopulationUpdated (Variables|Default|GetAC_Population) (EventDispatchers|CreateEvent :!event VisualSetPopulation))
        (if (Networking|IsServer)
          (Default|Inject (Variables|Default|GetAC_Population) (Math|Conversions|ToFloat(Integer) (Variables|InitialExposedValues|GetInitialPopulation)))
          (else
            (Visual|VisualSetPopulation (Variables|InitialExposedValues|GetInitialPopulation))))))
    (:then_4
      (if true ; Upgrade Bind/Set
        (EventDispatchers|BindEventtoCampUpdated (Variables|Default|GetAC_Upgrade) (EventDispatchers|CreateEvent :!event VisualSetTypeandLevel))
        (if (Networking|IsServer)
          (Default|SetCampandUpgrade (Variables|Default|GetAC_Upgrade) (Variables|InitialExposedValues|GetInitialCamp))
          (else
            (Visual|VisualSetTypeandLevel (.type _initialcamp) (.level _initialcamp) "NewEnumerator0")))))
    (:then_5
      (if true ; UpdateZOrder
        (CallFunction|UpdateZOrder (Variables|Default|GetVisualSet))))))

(fn ConstructionScript
  (CallFunction|InitialVisualValues))

(fn VisualSetTypeandLevel
  (params (Type :type Gameplay%20Tag%20Structure) (Level :type Integer) (State :type ECampRunStates%20Enum :default "NewEnumerator0"))
  (Utilities|FlowControl|Sequence
    (:then_0
      (if (Utilities|Enum|Equal(Enum) State "NewEnumerator2")
        (LocalVariables|Set_Sprite "/Game/Tiny/Art/Game/Sprites/SPR_Camp_Construction.SPR_Camp_Construction")
        (else
          (|SwitchGameplayTag Type
            (:Camp.House
              (switch int Level
                (:1
                  (LocalVariables|Set_Sprite "/Game/Tiny/Art/Game/Sprites/SPR_Camp_House_01.SPR_Camp_House_01"))
                (:2
                  (LocalVariables|Set_Sprite "/Game/Tiny/Art/Game/Sprites/SPR_Camp_House_02.SPR_Camp_House_02"))
                (:3
                  (LocalVariables|Set_Sprite "/Game/Tiny/Art/Game/Sprites/SPR_Camp_House_03.SPR_Camp_House_03"))
                (:4
                  (LocalVariables|Set_Sprite "/Game/Tiny/Art/Game/Sprites/SPR_Camp_House_04.SPR_Camp_House_04"))
                (:5
                  (LocalVariables|Set_Sprite "/Game/Tiny/Art/Game/Sprites/SPR_Camp_House_05.SPR_Camp_House_05"))))
            (:Camp.Tower
              (switch int Level
                (:1
                  (LocalVariables|Set_Sprite "/Game/Tiny/Art/Game/Sprites/SPR_Camp_Tower_01.SPR_Camp_Tower_01"))
                (:2
                  (LocalVariables|Set_Sprite "/Game/Tiny/Art/Game/Sprites/SPR_Camp_Tower_02.SPR_Camp_Tower_02"))
                (:3
                  (LocalVariables|Set_Sprite "/Game/Tiny/Art/Game/Sprites/SPR_Camp_Tower_03.SPR_Camp_Tower_03"))
                (:4
                  (LocalVariables|Set_Sprite "/Game/Tiny/Art/Game/Sprites/SPR_Camp_Tower_04.SPR_Camp_Tower_04"))
                (:5
                  (LocalVariables|Set_Sprite "/Game/Tiny/Art/Game/Sprites/SPR_Camp_Tower_05.SPR_Camp_Tower_05"))))
            (:Camp.Forge
              (switch int Level
                (:1
                  (LocalVariables|Set_Sprite "/Game/Tiny/Art/Game/Sprites/SPR_Camp_Forge_01.SPR_Camp_Forge_01"))
                (:2
                  (LocalVariables|Set_Sprite "/Game/Tiny/Art/Game/Sprites/SPR_Camp_Forge_02.SPR_Camp_Forge_02"))
                (:3
                  (LocalVariables|Set_Sprite "/Game/Tiny/Art/Game/Sprites/SPR_Camp_Forge_03.SPR_Camp_Forge_03"))
                (:4
                  (LocalVariables|Set_Sprite "/Game/Tiny/Art/Game/Sprites/SPR_Camp_Forge_04.SPR_Camp_Forge_04"))
                (:5
                  (LocalVariables|Set_Sprite "/Game/Tiny/Art/Game/Sprites/SPR_Camp_Forge_05.SPR_Camp_Forge_05"))))))))
    (:then_1
      (Rendering|Components|Sprite|SetSprite (Variables|Components|GetSPR_Camp) (LocalVariables|Get_Sprite)))))

(fn CampTypeComponentsAdd
  (bind _ac_upgrade (Variables|Default|GetAC_Upgrade))
  (bind (_type _level) (Default|GetCamp _ac_upgrade))
  (|SwitchGameplayTag _type
    (:Camp.House
      (if (== (Default|GetTeamValue (Variables|Default|GetAC_Team)) 0) ; Neutral team exception.
        (bind _returnvalue (Game|AddComponentbyClass "/Game/Tiny/Blueprints/Components/AC_GrowNeutral.AC_GrowNeutral_C" (Variables|Default|GetAC_Upgrade) (Variables|Default|GetAC_Population))) ; Ac_Grow
        (Utilities|Array|Add (Variables|Default|GetCampTypeComponents) _returnvalue)
        (Default|StartGrowing _returnvalue)
        (else
          (bind _returnvalue_2 (Game|AddComponentbyClass "/Game/Tiny/Blueprints/Components/AC_Grow.AC_Grow_C" (Variables|Default|GetAC_Upgrade) (Variables|Default|GetAC_Population))) ; Ac_Grow
          (Utilities|Array|Add (Variables|Default|GetCampTypeComponents) _returnvalue_2)
          (Default|StartGrowing _returnvalue_2))))
    (:Camp.Tower
      (bind _returnvalue_3 (AddComponent|AddSphereComponent false)) ; Sphere
      (Utilities|Array|Add (Variables|Default|GetCampTypeComponents) _returnvalue_3)
      (bind _returnvalue_4 (Game|AddComponentbyClass "/Game/Tiny/Blueprints/Components/AC_Shoot.AC_Shoot_C" _returnvalue_3 self)) ; AC_Shoot
      (Utilities|Array|Add (Variables|Default|GetCampTypeComponents) _returnvalue_4)
      (Default|ActivateSensingSphere _returnvalue_4 _level))))

(fn CampTypeComponentsRemove
  (for _array_element (Variables|Default|GetCampTypeComponents)
    (Components|DestroyComponent _array_element))
  (Utilities|Array|Clear (Variables|Default|GetCampTypeComponents)))

(fn VisualSetPopulation
  (params (Value :type Integer))
  (if true ; Widget
    (Default|SetPopulation (Variables|Refs|GetWBP_CampOverlay) Value)))

(fn SetIndex
  (params (NewValue :type Integer))
  (Variables|Replicated|SetIndex NewValue))

(fn GetIndex
  (return (Variables|Replicated|GetIndex)))

(fn GetDebugText
  (bind _ac_population (Variables|Default|GetAC_Population))
  (bind _ac_upgrade (Variables|Default|GetAC_Upgrade))
  (bind (_count _value) (Default|GetDebugText _ac_population))
  (bind (_camptype _camplevel _runstate _upgradeatack _upgradedefense _upgradenextcost _upgradenexttime) (Default|GetDebugText _ac_upgrade))
  (return (Utilities|Text|ToText(String) (Utilities|GetDisplayName self)) (Utilities|Text|ToText(Integer) (Variables|Replicated|GetIndex)) _count _value (Default|GetDebugText (Variables|Default|GetAC_Team)) _camptype _camplevel _runstate _upgradeatack _upgradedefense _upgradenextcost _upgradenexttime))

(fn VisualSetGrowLimit
  (if true ; Widget
    (bind _upgradegrow (CallFunction|GetDTGrowbyLevel (.Level (Default|GetCamp (Variables|Default|GetAC_Upgrade)))))
    (Default|SetGrowMax (Variables|Refs|GetWBP_CampOverlay) (.maxcount _upgradegrow) false)))

(fn VisualSetTeam
  (params (Team :type Integer))
  (Sprite|SetSpriteColor (Variables|Components|GetSPR_Camp) (CallFunction|GetTeamColor Team)))