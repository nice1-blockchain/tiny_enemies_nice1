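; AC_ObserverGlobal is an observer component that temporarily registers its team as watching every BP_Camp in the level.
; On StartObserving, the server caches all camp actors and adds the ACTeam value to each through MCAddWatchingTeam.
; After the Duration from the observer values, or on EndPlay, EndCycle removes that team from the cached camps and clears the list.
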(event Custom|EndCycle
  (if (Networking|IsServer)
    (for _array_element (Variables|Default|GetCurrentCamps)
      (Default|MCRemoveWatchingTeam _array_element (Default|GetTeamValue (Variables|Default|GetAC_Team))))
    (Utilities|Array|Clear (Variables|Default|GetCurrentCamps))))

(event Custom|StartObserving
  (if (Networking|IsServer)
    (Utilities|FlowControl|Sequence
      (:then_0
        (if true
          (bind _outactors (Actor|GetAllActorsOfClass "/Game/Tiny/Blueprints/BP_Camp.BP_Camp_C"))
          (for _array_element _outactors
            (Utilities|Array|Add (Variables|Default|GetCurrentCamps) _array_element)
            (Default|MCAddWatchingTeam _array_element (Default|GetTeamValue (Variables|Default|GetAC_Team))))))
      (:then_1
        (if true
          (Utilities|FlowControl|Delay (.Duration (CallFunction|GetObserverValues)))
          (CallFunction|EndCycle))))))

(event EventEndPlay
  (params (EndPlayReason :type EEndPlayReason%20Enum :default "Destroyed"))
  (CallFunction|EndCycle))