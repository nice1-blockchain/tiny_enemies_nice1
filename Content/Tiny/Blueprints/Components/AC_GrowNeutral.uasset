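; Actor component that periodically regrows a neutral's population, capped at the whole-number population recorded when growth starts.
; A looping timer, started on BeginPlay, injects an amount into ACPopulation scaled by a curve of the current fill ratio, clamped to that cap.
; Ticks act only while the game state is playing and no start-delay timer runs.
; SetGrowStartDelay pauses growth through that one-shot timer, while StopGrowing clears the looping timer.
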(event Custom|StartGrowing
  (Variables|Default|SetGrowMaxFixedLimit (.Truncated (Default|GetValue (Variables|Default|GetAC_Population))))
  (bind _returnvalue (Utilities|Time|SetTimerbyEvent (delegate Custom|GrowTick) (.Cadence (CallFunction|GetGrowNeutralValues)) true))
  (Variables|Default|SetGrowTimer _returnvalue))

(event Custom|StopGrowing
  (if (Utilities|Time|IsValidTimerHandle (Variables|Default|GetGrowTimer))
    (Utilities|Time|ClearandInvalidateTimerbyHandle (Variables|Default|GetGrowTimer))
    (Variables|Default|SetGrowTimer "")))

(event Custom|GrowTick
  (bind _amount (CallFunction|GetGrowNeutralValues))
  (bind _ac_population (Variables|Default|GetAC_Population))
  (bind _c_growcurve (Variables|Default|GetC_GrowCurve))
  (bind _growmaxfixedlimit (Variables|Default|GetGrowMaxFixedLimit))
  (bind _returnvalue (Math|Conversions|ToFloat(Integer) _growmaxfixedlimit))
  (bind _value (Default|GetValue _ac_population))
  (bind _returnvalue_2 (/ _value _returnvalue))
  (bind _returnvalue_3 (Math|Curves|GetFloatValue _c_growcurve _returnvalue_2))
  (bind _returnvalue_4 (* _amount _returnvalue_3))
  (bind _asbp_gs_game (CallFunction|GetGSGame))
  (if (and (Default|IsPlaying _asbp_gs_game) (not (Utilities|Time|IsValidTimerHandle (Variables|Default|GetStartDelayTimer))))
    (if (<= (+ _returnvalue_4 _value) _returnvalue)
      (Default|Inject (Variables|Default|GetAC_Population) _returnvalue_4)
      (else
        (Default|Inject (Variables|Default|GetAC_Population) (- _returnvalue _value))))))

(event Custom|SetGrowStartDelay
  (bind _returnvalue (Utilities|Time|SetTimerbyEvent (delegate Custom|Nothing) (.StartDelay (CallFunction|GetGrowNeutralValues))))
  (Variables|Default|SetStartDelayTimer _returnvalue))

(event Custom|Nothing
  (Utilities|Time|InvalidateTimerHandle (Variables|Default|GetStartDelayTimer))
  (Variables|Default|SetStartDelayTimer ""))

(event EventBeginPlay
  (CallFunction|StartGrowing))