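; Actor component that periodically grows a camp's population while the game is playing, up to a cap set by the camp's level.
; A looping timer, started and stopped by events, runs the growth tick at a configurable cadence.
; Each tick looks up amount and max count by level, scales the amount with a curve sampled at the current fill ratio, and injects it into the population component, clamped to the maximum.
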(event Custom|GrowTick
  (bind _ac_population (Variables|Default|GetAC_Population))
  (bind _value (Default|GetValue _ac_population))
  (bind _asbp_gs_game (CallFunction|GetGSGame))
  (if (Default|CheckPlaying _asbp_gs_game)
    (bind _upgradegrow (CallFunction|GetDTGrowbyLevel (.Level (Default|GetCamp (Variables|Default|GetAC_Upgrade)))))
    (if (< _value (.maxcount _upgradegrow))
      (if (<= (+ (* (.amount _upgradegrow) (Math|Curves|GetFloatValue (Variables|Default|GetC_GrowCurve) (/ _value (Math|Conversions|ToFloat(Integer) (.maxcount _upgradegrow))))) _value) (Math|Conversions|ToFloat(Integer) (.maxcount _upgradegrow)))
        (Default|Inject (Variables|Default|GetAC_Population) (* (.amount _upgradegrow) (Math|Curves|GetFloatValue (Variables|Default|GetC_GrowCurve) (/ _value (Math|Conversions|ToFloat(Integer) (.maxcount _upgradegrow))))))
        (else
          (Default|Inject (Variables|Default|GetAC_Population) (- (Math|Conversions|ToFloat(Integer) (.maxcount _upgradegrow)) _value)))))))

(event Custom|StartGrowing
  (bind _returnvalue (Utilities|Time|SetTimerbyEvent (delegate Custom|GrowTick) (CallFunction|GetGrowCadence) true))
  (Variables|Default|SetGrowTimer _returnvalue))

(event Custom|StopGrowing
  (if (Utilities|Time|IsValidTimerHandle (Variables|Default|GetGrowTimer))
    (Utilities|Time|ClearandInvalidateTimerbyHandle (Variables|Default|GetGrowTimer))
    (Variables|Default|SetGrowTimer "")))