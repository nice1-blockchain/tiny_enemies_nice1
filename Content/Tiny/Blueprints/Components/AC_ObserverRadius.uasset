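; Component on a BP_Camp that marks nearby camps as watched by its team within an observer radius.
; On BeginPlay, the server multicasts a watch decal sized to the radius and spawns a hidden cylinder, both Y-scaled to match perspective.
; A one-time overlap query on the cylinder registers the team with each camp found.
; EndCycle, also run on EndPlay, removes the decal and those watch registrations.
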(event Custom|EndCycle
  (CallFunction|MCDecalDestroy)
  (if (Networking|IsServer)
    (for _array_element (Variables|Default|GetCurrentCamps)
      (Default|MCRemoveWatchingTeam _array_element (Default|GetTeamValue (Variables|Default|GetAC_Team))))
    (Utilities|Array|Clear (Variables|Default|GetCurrentCamps))))

(event Custom|StartObserving
  (bind _radius (CallFunction|GetObserverValues))
  (bind _returnvalue (* _radius 2.0))
  (if (Networking|IsServer)
    (Utilities|FlowControl|Sequence
      (:then_0
        (if true
          (CallFunction|MCDecalCreate (.Radius (CallFunction|GetObserverValues)))))
      (:then_1
        (if true
          (bind _returnvalue_2 (Game|AddComponentbyClass (.AsBP%20Camp (Utilities|Casting|CastToBP_Camp (Components|GetOwner))) "/Script/Engine.StaticMeshComponent" false))
          (bind _output_get (Variables|Default|SetSensingMesh _returnvalue_2))
          (Components|StaticMesh|SetStaticMesh _output_get "/Game/Tiny/Art/SM_Cylinder.SM_Cylinder")
          (Development|SetHiddeninGame (Variables|Default|GetSensingMesh) true false)))
      (:then_2
        (if true
          (Transformation|SetWorldScale3D (Variables|Default|GetSensingMesh) (Math|Vector|MakeVector _returnvalue (* _returnvalue (CallFunction|GetYScaletoMatchPerspective)) _returnvalue))
          (Collision|SetCollisionResponsetoAllChannels (Variables|Default|GetSensingMesh) "ECR_Ignore")
          (Collision|SetCollisionObjectType (Variables|Default|GetSensingMesh) "ECC_WorldStatic")
          (Collision|SetCollisionResponsetoChannel (Variables|Default|GetSensingMesh) "ECC_WorldDynamic" "ECR_Overlap")))
      (:then_3
        (if true
          (for _array_element (Collision|GetOverlappingActors (Variables|Default|GetSensingMesh) "/Game/Tiny/Blueprints/BP_Camp.BP_Camp_C" :!class /Script/Engine.PrimitiveComponent)
            (bind _asbp_camp (Utilities|Casting|CastToBP_Camp _array_element))
            (Utilities|Array|Add (Variables|Default|GetCurrentCamps) _asbp_camp)
            (Default|MCAddWatchingTeam _asbp_camp (Default|GetTeamValue (Variables|Default|GetAC_Team)))))))))

(event Custom|MC_DecalCreate
  (params (Radius :type Float%20%28double-precision%29))
  (bind _returnvalue (Math|Float|MakeLiteralFloat 256.0))
  (bind _returnvalue_2 (/ Radius _returnvalue))
  (Utilities|IsValid (Variables|Default|GetAC_DecalComponent)
    (:Is%20Valid
      (Default|DestroySelfComponent (.AsBP%20Camp (Utilities|Casting|CastToBP_Camp (Components|GetOwner))) (Variables|Default|GetAC_DecalComponent)))
    (:Is%20Not%20Valid
      _))
  (bind _returnvalue_3 (Game|AddComponentbyClass (.AsBP%20Camp (Utilities|Casting|CastToBP_Camp (Components|GetOwner))) "/Script/Engine.DecalComponent" false (Math|Transform|MakeTransform "0, 0, 0" "90.000000, 0, 0" (Math|Vector|MakeVector _returnvalue_2 (* _returnvalue_2 (CallFunction|GetYScaletoMatchPerspective)) _returnvalue_2))))
  (bind _output_get (Variables|Default|SetAC_DecalComponent _returnvalue_3))
  (Rendering|Components|Decal|SetDecalMaterial _output_get "/Game/Tiny/Art/MI_Decal_Watch.MI_Decal_Watch"))

(event Custom|MC_DecalDestroy
  (Utilities|IsValid (Variables|Default|GetAC_DecalComponent)
    (:Is%20Valid
      (Default|DestroySelfComponent (.AsBP%20Camp (Utilities|Casting|CastToBP_Camp (Components|GetOwner))) (Variables|Default|GetAC_DecalComponent)))))

(event EventEndPlay
  (params (EndPlayReason :type EEndPlayReason%20Enum :default "Destroyed"))
  (CallFunction|EndCycle))

(event EventBeginPlay
  (CallFunction|StartObserving))