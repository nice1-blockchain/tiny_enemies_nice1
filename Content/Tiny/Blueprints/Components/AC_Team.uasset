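; AC_Team is an actor component that stores an integer team value for its owning actor.
; Getter and setter functions read and write TeamValue, and its RepNotify broadcasts the TeamUpdated dispatcher with the new value.
; A debug function returns the team value as text.
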(fn GetTeamValue
  (return (Variables|Private|GetTeamValue)))

(fn SetTeamValue
  (params (NewValue :type Integer))
  (Variables|Private|SetTeamValue NewValue))

(fn OnRepTeamValue
  (Default|CallTeamUpdated (Variables|Private|GetTeamValue)))

(fn GetDebugText
  (return (Utilities|Text|ToText(Integer) (Variables|Private|GetTeamValue))))