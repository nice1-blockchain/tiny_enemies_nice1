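; Shooting component that lets a BP_Camp act as a tower, killing enemy wave units within range.
; On the server it builds a hidden cylinder sensor and multicasts a range decal, both sized from level-based shoot data with perspective-corrected Y scale.
; Overlaps maintain the sensed-unit list and start or stop a looping cadence timer.
; Each shot instantly kills a shuffled enemy picked by a widening band around 70% of range, then notifies its wave.
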(event Custom|ActivateSensingSphere
  (if (Networking|IsServer)
    (Utilities|FlowControl|Sequence
      (:then_0
        (bind _returnvalue (Game|AddComponentbyClass (Variables|Default|GetBP_Camp_Parent) "/Script/Engine.StaticMeshComponent" false))
        (bind _output_get (Variables|Default|SetSensingMesh _returnvalue))
        (Components|StaticMesh|SetStaticMesh _output_get "/Game/Tiny/Art/SM_Cylinder.SM_Cylinder")
        (Development|SetHiddeninGame (Variables|Default|GetSensingMesh) true false))
      (:then_1
        (bind _upgradeshoot (CallFunction|GetDTShoot (.level (Default|GetCampKey (Variables|/Game/Tiny/Blueprints/BP_Camp.BP_Camp_C|GetAC_State (Variables|Default|GetBP_Camp_Parent))))))
        (bind _output_get_2 (Variables|Default|SetUpgradeShoot _upgradeshoot))
        (Utilities|FlowControl|Sequence
          (:then_0
            (Transformation|SetWorldScale3D (Variables|Default|GetSensingMesh) (Math|Vector|MakeVector (* (.MaxRange (Utilities|Struct|BreakSShoot _output_get_2)) 2.0) (* (* (.MaxRange (Utilities|Struct|BreakSShoot _output_get_2)) 2.0) (CallFunction|GetYScaletoMatchPerspective)) (* (.MaxRange (Utilities|Struct|BreakSShoot _output_get_2)) 2.0)))
            (Collision|BindEventtoOnComponentBeginOverlap (Variables|Default|GetSensingMesh) (EventDispatchers|CreateEvent :!event Custom|BeginOverlap))
            (Collision|BindEventtoOnComponentEndOverlap (Variables|Default|GetSensingMesh) (EventDispatchers|CreateEvent :!event Custom|EndOverlap)))))
      (:then_2
        (CallFunction|MCDecalCreate (.MaxRange (Utilities|Struct|BreakSShoot (Variables|Default|GetUpgradeShoot))))))))

(event Custom|BeginOverlap
  (params (OverlappedComponent :type Primitive%20Component%20Object%20Reference) (OtherActor :type Actor%20Object%20Reference) (OtherComp :type Primitive%20Component%20Object%20Reference) (OtherBodyIndex :type Integer) (bFromSweep :type Boolean) (SweepResult :type Hit%20Result%20Structure%20%28by%20ref%29))
  (if (Networking|IsServer)
    (bind _asbp_unit (Utilities|Casting|CastToBP_Unit OtherActor))
    (Utilities|Array|AddUnique (Variables|Default|GetSensedUnits) _asbp_unit)
    (if (CallFunction|GetShootEnable)
      (CallFunction|StartShooting)
      (else
        (Development|PrintString "Gloabal: Shoot disable.")))))

(event Custom|EndOverlap
  (params (OverlappedComponent :type Primitive%20Component%20Object%20Reference) (OtherActor :type Actor%20Object%20Reference) (OtherComp :type Primitive%20Component%20Object%20Reference) (OtherBodyIndex :type Integer))
  (if (Networking|IsServer)
    (bind _asbp_unit (Utilities|Casting|CastToBP_Unit OtherActor))
    (Utilities|Array|RemoveItem (Variables|Default|GetSensedUnits) _asbp_unit)
    (Utilities|FlowControl|RetriggerableDelay 0.15)
    (if (Utilities|Array|IsEmpty (Variables|Default|GetSensedUnits))
      (CallFunction|StopShooting))))

(event Custom|StartShooting
  (if (and (not (Utilities|Time|IsValidTimerHandle (Variables|Default|GetCycleTimer))) (Variables|Default|GetbActive))
    (bind _returnvalue (Utilities|Time|SetTimerbyEvent (EventDispatchers|CreateEvent :!event Custom|TimeToShoot) (.Cadence (Utilities|Struct|BreakSShoot (Variables|Default|GetUpgradeShoot))) true))
    (Variables|Default|SetCycleTimer _returnvalue)
    (CallFunction|TimetoShoot) ; First intant shoot.
  ))

(event Custom|TimeToShoot
  (bind (_bvalid _unit) (Private|TargetSelection))
  (if _bvalid
    (Default|SetKilled _unit)
    (Default|UnitKilled (Variables|/Game/Tiny/Blueprints/BP_Unit.BP_Unit_C|GetBP_Wave_Parent _unit) (Default|GetIndex (Variables|Default|GetBP_Camp_Parent)) (Variables|/Game/Tiny/Blueprints/BP_Unit.BP_Unit_C|GetIndex _unit))))

(event Custom|StopShooting
  (if (Utilities|Time|IsValidTimerHandle (Variables|Default|GetCycleTimer))
    (Utilities|Time|ClearandInvalidateTimerbyHandle (Variables|Default|GetCycleTimer))
    (Variables|Default|SetCycleTimer "")))

(event Custom|MC_DecalCreate
  (params (Range :type Float%20%28double-precision%29))
  (bind _returnvalue (Math|Float|MakeLiteralFloat 256.0))
  (bind _returnvalue_2 (/ Range _returnvalue))
  (bind _returnvalue_3 (Game|AddComponentbyClass (.AsBP%20Camp (Utilities|Casting|CastToBP_Camp (Components|GetOwner))) "/Script/Engine.DecalComponent" false (Math|Transform|MakeTransform "0, 0, 0" "90.000000, 0, 0" (Math|Vector|MakeVector _returnvalue_2 (* _returnvalue_2 (CallFunction|GetYScaletoMatchPerspective)) _returnvalue_2))))
  (bind _output_get (Variables|Default|SetAC_DecalComponent _returnvalue_3))
  (Rendering|Components|Decal|SetDecalMaterial _output_get "/Game/Tiny/Art/MI_Decal_Tower.MI_Decal_Tower"))

(event EventEndPlay
  (params (EndPlayReason :type EEndPlayReason%20Enum :default "Destroyed"))
  (Default|DestroySelfComponent (.AsBP%20Camp (Utilities|Casting|CastToBP_Camp (Components|GetOwner))) (Variables|Default|GetAC_DecalComponent)))

(event EventBeginPlay
  (CallFunction|ActivateSensingSphere))

(fn TargetSelection
  (bind _returnvalue (Math|Float|MakeLiteralFloat 0.7))
  (Utilities|FlowControl|Sequence
    (:then_0
      (if true
        (for _array_element (Variables|Default|GetSensedUnits)
          (if (and (!= (Default|GetTeamValue (Variables|/Game/Tiny/Blueprints/BP_Camp.BP_Camp_C|GetAC_Team (Variables|Default|GetBP_Camp_Parent))) (Default|GetTeamValue (Variables|/Game/Tiny/Blueprints/BP_Wave.BP_Wave_C|GetAC_Team (Variables|/Game/Tiny/Blueprints/BP_Unit.BP_Unit_C|GetBP_Wave_Parent _array_element)))) (not (Default|GetKilled _array_element)))
            (Utilities|Array|Add (LocalVariables|Get_ValidFiltered) _array_element)))
        (Utilities|Array|Shuffle (LocalVariables|Get_ValidFiltered))))
    (:then_2
      (if true
        (if (Utilities|Array|IsValidIndex (LocalVariables|Get_ValidFiltered))
          (while (not (Utilities|IsValid (LocalVariables|Get_UnitCurrentSelected)))
            (for _array_element_2 (LocalVariables|Get_ValidFiltered)
              (if (and (!= (Default|GetTeamValue (Variables|/Game/Tiny/Blueprints/BP_Camp.BP_Camp_C|GetAC_Team (Variables|Default|GetBP_Camp_Parent))) (Default|GetTeamValue (Variables|/Game/Tiny/Blueprints/BP_Wave.BP_Wave_C|GetAC_Team (Variables|/Game/Tiny/Blueprints/BP_Unit.BP_Unit_C|GetBP_Wave_Parent _array_element_2)))) (not (Default|GetKilled _array_element_2)))
                (if (and (> (Math|Vector|VectorLength (- (Transformation|GetActorLocation _array_element_2) (Transformation|GetWorldLocation (Variables|Default|GetSensingMesh)))) (* (.MaxRange (Utilities|Struct|BreakSShoot (Variables|Default|GetUpgradeShoot))) (- _returnvalue (LocalVariables|Get_Range)))) (< (Math|Vector|VectorLength (- (Transformation|GetActorLocation _array_element_2) (Transformation|GetWorldLocation (Variables|Default|GetSensingMesh)))) (* (.MaxRange (Utilities|Struct|BreakSShoot (Variables|Default|GetUpgradeShoot))) (+ _returnvalue (LocalVariables|Get_Range)))))
                  (LocalVariables|Set_UnitCurrentSelected _array_element_2))))
            (LocalVariables|Set_Range (+ (LocalVariables|Get_Range) (LocalVariables|Get_Range))))
          (return true (LocalVariables|Get_UnitCurrentSelected))
          (else
            (return false 0)))))))

(fn GetDebugText
  (bind _upgradeshoot (Variables|Default|GetUpgradeShoot))
  (bind (_cadence _maxrange) (Utilities|Struct|BreakSShoot _upgradeshoot))
  (Utilities|FlowControl|Sequence
    (:then_0
      (for _array_element (Variables|Default|GetSensedUnits)
        (LocalVariables|Set_SensedUnits (Utilities|String|Append (LocalVariables|Get_SensedUnits) (Utilities|GetDisplayName _array_element) " "))))
    (:then_1
      (return (Utilities|Text|ToText(Float) _cadence "HalfToEven") (Utilities|Text|ToText(Float) _maxrange "HalfToEven") (Utilities|Text|ToText(Float) (Utilities|Time|GetTimerRemainingTimebyHandle (Variables|Default|GetCycleTimer)) "HalfToEven") (Utilities|Text|ToText(String) (LocalVariables|Get_SensedUnits))))))

(fn SetActiveSwitch
  (params (bActive :type Boolean))
  (Variables|Default|SetbActive bActive))