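; AC_Observer is a component that lets a BP_Camp watch other camps within a radius for its team.
; On start it adds a sensing sphere to the owner, then registers its team as a watcher on the camps overlapping at that moment.
; MC_ events create and destroy a range decal with perspective-corrected Y scale.
; On EndPlay the server unregisters the team and removes the sphere and decal.
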(event Custom|AddSensingSphere
  (bind _radius (Variables|Default|GetRadius))
  (Utilities|FlowControl|Sequence
    (:then_0
      (if true
        (Development|PrintString "Observer init.")))
    (:then_1
      (if true
        (bind _asbp_camp (Utilities|Casting|CastToBP_Camp (Components|GetOwner)))
        (bind _returnvalue (Game|AddComponentbyClass _asbp_camp "/Script/Engine.SphereComponent" false))
        (bind _output_get (Variables|Default|SetSensingSphere _returnvalue))
        (Components|Sphere|SetSphereRadius _output_get _radius true)
        (CallFunction|MCDecalCreate _radius)))
    (:then_2
      (if true
        (for _array_element (Collision|GetOverlappingActors (Variables|Default|GetSensingSphere) "/Game/Tiny/Blueprints/BP_Camp.BP_Camp_C" :!class /Script/Engine.PrimitiveComponent)
          (bind _asbp_camp_2 (Utilities|Casting|CastToBP_Camp _array_element))
          (Utilities|Array|Add (Variables|Default|GetCurrentCamps) _asbp_camp_2)
          (Default|AddWatchingTeam _asbp_camp_2 (Default|GetTeamValue (Variables|Default|GetAC_Team))))))))

(event Custom|StartObserving
  (CallFunction|AddSensingSphere))

(event Custom|MC_DecalCreate
  (params (Range :type Float%20%28double-precision%29))
  (bind _returnvalue (Math|Float|MakeLiteralFloat 256.0))
  (bind _returnvalue_2 (/ Range _returnvalue))
  (bind _returnvalue_3 (Game|AddComponentbyClass (.AsBP%20Camp (Utilities|Casting|CastToBP_Camp (Components|GetOwner))) "/Script/Engine.DecalComponent" false (Math|Transform|MakeTransform "0, 0, 0" "90.000000, 0, 0" (Math|Vector|MakeVector _returnvalue_2 (* _returnvalue_2 (CallFunction|GetYScaletoMatchPerspective)) _returnvalue_2))))
  (bind _output_get (Variables|Default|SetAC_DecalComponent _returnvalue_3))
  (Rendering|Components|Decal|SetDecalMaterial _output_get "/Game/Tiny/Art/MI_Decal_Watch.MI_Decal_Watch"))

(event Custom|MC_DecalDestroy
  (Default|DestroySelfComponent (.AsBP%20Camp (Utilities|Casting|CastToBP_Camp (Components|GetOwner))) (Variables|Default|GetAC_DecalComponent)))

(event EventEndPlay
  (params (EndPlayReason :type EEndPlayReason%20Enum :default "Destroyed"))
  (if (Networking|IsServer)
    (Utilities|FlowControl|Sequence
      (:then_0
        (if true
          (for _array_element (Variables|Default|GetCurrentCamps)
            (Default|RemoveWatchingTeam _array_element (Default|GetTeamValue (Variables|Default|GetAC_Team))))
          (Utilities|Array|Clear (Variables|Default|GetCurrentCamps))))
      (:then_1
        (if true
          (Components|DestroyComponent (Variables|Default|GetSensingSphere))))
      (:then_2
        (CallFunction|MCDecalDestroy)))))