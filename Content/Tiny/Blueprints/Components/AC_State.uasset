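; AC_State is a component that holds a camp's state: its type and level key, matching stat values and a run mode.
; On BeginPlay and on every upgrade or type reset, it looks up the camp value by key from a data table.
; Upgrades proceed only if the target level's lookup is valid, and resets return to level 1.
; RepNotifies on the value and run mode call StateValueUpdated.
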(event EventBeginPlay
  (GetSet|SetCampKeyandValue (Variables|Default|GetKey)))

(fn SetCampKeyandValue
  (params (CampKey :type S%20Camp%20Key%20Structure))
  (bind _output_get (Variables|Default|SetKey CampKey))
  (bind (_valid _value) (CallFunction|GetDTCampValue _output_get))
  (if _valid
    (Variables|Default|SetValue _value)))

(fn GetCampKey
  (return (Variables|Default|GetKey)))

(fn GetCampValue
  (return (Variables|Default|GetValue)))

(fn GetDebugText
  (bind _value (Variables|Default|GetValue))
  (bind _key (Variables|Default|GetKey))
  (return (Utilities|Text|ToText(Name) (GameplayTags|GetTagName (.type _key))) (Utilities|Text|ToText(Integer) (.level _key)) (Utilities|Text|ToText(String) (Utilities|String|EnumtoString (Variables|Default|GetRunMode))) (Utilities|Text|ToText(Float) (.atack _value) "HalfToEven") (Utilities|Text|ToText(Float) (.defense _value) "HalfToEven") (Utilities|Text|ToText(Integer) (.upgradecost _value)) (Utilities|Text|ToText(Float) (.upgradetime _value) "HalfToEven")))

(fn OnRepValue
  (Default|CallStateValueUpdated))

(fn CanbeUpgraded
  (params (Offset :type Integer))
  (bind _key (Variables|Default|GetKey))
  (bind _valid (CallFunction|GetDTCampValue (Utilities|Struct|MakeSCampKey (.type _key) (+ Offset (.level _key)))))
  (return _valid))

(fn UpgradeOffsetif
  (params (Offset :type Integer))
  (bind _key (Variables|Default|GetKey))
  (bind _valid (Abilities|CanbeUpgraded Offset))
  (if _valid
    (GetSet|SetCampKeyandValue (Utilities|Struct|MakeSCampKey (.type _key) (+ (.level _key) Offset)))
    (return)))

(fn CanbeResetto
  (params (Type :type Gameplay%20Tag%20Structure))
  (return (!= Type (.Type (Utilities|Struct|BreakSCampKey (Variables|Default|GetKey))))))

(fn Resetto
  (params (Type :type Gameplay%20Tag%20Structure))
  (GetSet|SetCampKeyandValue (Utilities|Struct|MakeSCampKey Type 1))
  (return))

(fn OnRepRunMode
  (Default|CallStateValueUpdated))

(fn GetRunMode
  (return (Variables|Default|GetRunMode)))

(fn SetRunMode
  (params (NewValue :type ERunMode%20Enum :default "NewEnumerator0"))
  (Variables|Default|SetRunMode NewValue))