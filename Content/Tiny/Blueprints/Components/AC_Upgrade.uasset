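; AC_Upgrade is an actor component that holds a camp's type, level and run state along with the upgrade stats for that level.
; Every camp change, from BeginPlay, level steps or type resets to level one, goes through SetCampAndUpgrade, which refreshes the stats via GetDTUpgrade.
; RunState uses a RepNotify to broadcast CampUpdated.
; Helpers expose level-limit checks and debug text.
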(event Custom|SetLevel
  (params (bDowngrade :type Boolean))
  (bind _camp (Variables|Default|GetCamp))
  (GetSet|SetCampandUpgrade (Utilities|Struct|MakeSCamp (.type _camp) (+ (.level _camp) (Math|Integer|SelectInt -1 1 bDowngrade)))))

(event Custom|SetResetTo
  (params (Type :type Gameplay%20Tag%20Structure))
  (GetSet|SetCampandUpgrade (Utilities|Struct|MakeSCamp Type 1)))

(event EventBeginPlay
  (GetSet|SetCampandUpgrade (Variables|Default|GetCamp)))

(fn SetRunState
  (params (NewValue :type ECampRunStates%20Enum :default "NewEnumerator0"))
  (Variables|Default|SetRunState NewValue))

(fn GetCamp
  (bind _camp (Variables|Default|GetCamp))
  (bind (_type _level) (Utilities|Struct|BreakSCamp _camp))
  (return _type _level (Variables|Default|GetRunState)))

(fn OnRepRunState
  (bind _camp (Variables|Default|GetCamp))
  (Default|CallCampUpdated (.type _camp) (.level _camp) (Variables|Default|GetRunState)))

(fn GetUpgrade
  (return (Variables|Default|GetUpgrade)))

(fn SetCampandUpgrade
  (params (Camp :type S%20Camp%20Structure))
  (bind _output_get (Variables|Default|SetCamp Camp))
  (bind _upgradecamp (CallFunction|GetDTUpgrade _output_get))
  (Variables|Default|SetUpgrade _upgradecamp))

(fn CanbeUpgraded
  (return (< (.Level (Utilities|Struct|BreakSCamp (Variables|Default|GetCamp))) (CallFunction|GetCampUpgradeMaxLevel))))

(fn CanbeDowngraded
  (return (> (.Level (Utilities|Struct|BreakSCamp (Variables|Default|GetCamp))) 1)))

(fn GetDebugText
  (bind _upgrade (Variables|Default|GetUpgrade))
  (bind _camp (Variables|Default|GetCamp))
  (return (Utilities|Text|ToText(Name) (GameplayTags|GetTagName (.type _camp))) (Utilities|Text|ToText(Integer) (.level _camp)) (Utilities|Text|ToText(String) (Utilities|String|EnumtoString (Variables|Default|GetRunState))) (Utilities|Text|ToText(Float) (.atack _upgrade) "HalfToEven") (Utilities|Text|ToText(Float) (.defense _upgrade) "HalfToEven") (Utilities|Text|ToText(Integer) (.nextcost _upgrade)) (Utilities|Text|ToText(Float) (.nexttime _upgrade) "HalfToEven")))