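; AC_Population is a component that stores a replicated population count as a float, with a truncated value for whole-number reads.
; Inject adds to the pool, and Extract removes a requested amount or drains what remains, reporting depletion.
; GetPercentageOfPopulation sizes a portion of the pool, clamped between wave send limits and the available population.
; Replication of the value fires a PopulationUpdated event, and debug text exposes both readings.
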(fn GetValue
  (bind _value (Variables|Private|GetValue))
  (return _value (Math|Float|Truncate _value)))

(fn Inject
  (params (Value :type Float%20%28double-precision%29))
  (Variables|Private|SetValue (+ (Variables|Private|GetValue) Value)))

(fn Extract
  (params (Value :type Float%20%28double-precision%29))
  (bind _bvalid (Public|HasEnough Value))
  (if _bvalid
    (bind _output_get (LocalVariables|Set_Extracted Value))
    (Variables|Private|SetValue (- (Variables|Private|GetValue) _output_get))
    (return false (LocalVariables|Get_Extracted))
    (else
      (LocalVariables|Set_Extracted (Variables|Private|GetValue))
      (Variables|Private|SetValue 0.0)
      (return true (LocalVariables|Get_Extracted)))))

(fn GetPercentageOfPopulation
  (params (Percent :type Integer))
  (bind _bvalid (Public|HasEnough 1.0))
  (if _bvalid
    (bind _output_get (LocalVariables|Set_Estimated (Math|Float|Clamp(Float) (* (Variables|Private|GetValue) (/ (Math|Conversions|ToFloat(Integer) Percent) 1e+02)) (Math|Conversions|ToFloat(Integer) (CallFunction|GetWaveSendMin)) (Math|Float|Min(Float) (Math|Conversions|ToFloat(Integer) (CallFunction|GetWaveSendMax)) (Variables|Private|GetValue)))))
    (bind _bvalid_2 (Public|HasEnough _output_get))
    (if _bvalid_2
      (return true (LocalVariables|Get_Estimated))
      (else
        (return true (Variables|Private|GetValue))))
    (else
      (return false 0.0))))

(fn HasEnough
  (params (Value :type Float%20%28double-precision%29))
  (return (<= Value (Variables|Private|GetValue))))

(fn OnRepValue
  (Default|CallPopulationUpdated))

(fn GetDebugText
  (return (Utilities|Text|ToText(Integer) (.Truncated (Public|GetValue))) (Utilities|Text|ToText(Float) (Variables|Private|GetValue) "HalfToEven")))